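; BP_Gong is an interactable gong that plays a sound and temporarily shifts the player's view to itself.
; Interact plays the gong sound at world origin, waits briefly, blends the view to the gong, holds, then calls ResetCamera to blend back to the player character.
; The box overlap is mostly stubbed: begin overlap does nothing, and end overlap prints a debug goodbye for INT_Player actors.
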(event `ResetCamera`
  (`PlayerController.SetViewTargetWithBlend` (`GameplayStatics.GetPlayerController` 0) (`GameplayStatics.GetPlayerCharacter` 0) 0.75 "VTBlend_Linear" 0.0 false))

(event `/Game/Blueprints/Interface/INT_Interact.Interact`
  (`GameplayStatics.PlaySoundAtLocation` "/Game/Almas_Assets/Sounds/Gong_sound_effect.Gong_sound_effect" (0.0 0.0 0.0) (struct) 1.0 1.0 0.0 null null null)
  (`KismetSystemLibrary.Delay` 2.5)
  (`PlayerController.SetViewTargetWithBlend` (`GameplayStatics.GetPlayerController` 0) self 2.0 "VTBlend_Cubic" 0.0 false)
  (`KismetSystemLibrary.Delay` 10.0)
  (`self.ResetCamera`))

(event `self.Box.OnComponentBeginOverlap`
  (params (OverlappedComponent :type "PrimitiveComponent Object Reference") (OtherActor :type "Actor Object Reference") (OtherComp :type "PrimitiveComponent Object Reference") (OtherBodyIndex :type Integer) (bFromSweep :type Boolean) (SweepResult :type "HitResult Structure (by ref)")))

(event `self.Box.OnComponentEndOverlap`
  (params (OverlappedComponent :type "PrimitiveComponent Object Reference") (OtherActor :type "Actor Object Reference") (OtherComp :type "PrimitiveComponent Object Reference") (OtherBodyIndex :type Integer))
  (if (`KismetSystemLibrary.DoesImplementInterface` OtherActor "/Game/Blueprints/Interface/INT_Player.INT_Player_C")
    (`KismetSystemLibrary.PrintString` "GoodBye")))

(fn `UserConstructionScript`)