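; BP_DummyTarget is a damageable dummy target that shows floating damage numbers and drops randomized weapons when destroyed.
; AnyDamage runs hits through CalculateDamages using damage types from BP_GlobalVariables and multiple health bars, marking depleted bars dead.
; Damage text is relayed through server and multicast-named events to the instigator's PlayerController.
; Once all bars are dead, a short delay precedes spawning loot-table weapons with rolled stat bonuses and destroying the actor.
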(event `Death`
  (bind (_location _rotation) (`/Game/BhandanaDesign/Actors/OBJ_CustomMacros.Get Loot Spawn Point` (`self.DefaultSceneRoot`)))
  (for _ (range 1 (+ (`/Game/BhandanaDesign/Actors/OBJ_CustomMacros.ROLL Number of Drops`) 1))
    (bind _returnvalue (`|SpawnActorFromClass` "/Game/BhandanaDesign/Actors/Weapons/Weaponpickup/BP_WeaponDrop_MASTER.BP_WeaponDrop_MASTER_C" (`KismetMathLibrary.MakeTransform` _location _rotation) "Undefined" "OverrideRootScale" null null))
    (set `/Game/BhandanaDesign/Actors/Weapons/Weaponpickup/BP_WeaponDrop_MASTER.Weapon Data` (`/Game/BhandanaDesign/Actors/OBJ_CustomMacros.ROLL Random Weapon From Drop Table With Unique Stats` (`self.Loot Table`) 25.0 25.0 20.0 20.0) _returnvalue)
    (`/Game/BhandanaDesign/Actors/Weapons/Weaponpickup/BP_WeaponDrop_MASTER.Visual Update` _returnvalue))
  (`self.K2_DestroyActor` self))

(event `RUNONSERVERCombatText`
  (params (damage :type "Float (double-precision)") (`font color` :type "Color Structure") (Instigator :type "Actor Object Reference"))
  (`self.MulticastCombatText` damage `font color` Instigator))

(event `MulticastCombatText`
  (params (damage :type "Float (double-precision)") (`Font Color` :type "Color Structure") (Instigator :type "Actor Object Reference"))
  (bind _asplayer_controller (cast `PlayerController` (`self.GetInstigatorController` Instigator)))
  (`/Game/BhandanaDesign/Actors/OBJ_CustomMacros.CreateDamageText` damage `Font Color` (`SceneComponent.K2_GetComponentLocation` (`self.DamageTextSpawnPoint`)) _asplayer_controller))

(event `self.ReceiveAnyDamage`
  (params (Damage :type "Float (single-precision)") (DamageType :type "DamageType Object Reference") (InstigatedBy :type "Controller Object Reference") (DamageCauser :type "Actor Object Reference"))
  (bind _hpbars (`self.HPBars`))
  (bind _deadhpbars (`self.deadHPBars`))
  (bind (_new_health _new_damage _text_color _hpbarindex) (`/Game/BhandanaDesign/Actors/OBJ_CustomMacros.CalculateDamages` Damage DamageType (`self.HPBars`) (`self.DamageTypes`))
    (:`Alive`
      (`self.RUNONSERVERCombatText` _new_damage _text_color DamageCauser))
    (:`Dead`
      (bind _structout (setmembers `/Game/BhandanaDesign/VariableData/Structs/ST_HPBar` :`StructRef` (`|GetArrayItem` _hpbars _hpbarindex) :`isDead` true))
      (`KismetArrayLibrary.Array_Set` _hpbars _hpbarindex _structout)
      (`/Engine/EditorBlueprintResources/StandardMacros.IncrementInt` _deadhpbars
        (:`  `
          (`self.RUNONSERVERCombatText` _new_damage _text_color DamageCauser)
          (if (>= _deadhpbars (`KismetArrayLibrary.Array_Length` _hpbars))
            (`KismetSystemLibrary.Delay` 0.2)
            (`self.Death`)))))))

(event `BeginCleanup`
  (params (ActorToDestroy :type "Actor Object Reference"))
  (`self.Cleanup` ActorToDestroy))

(event `Cleanup`
  (params (DeletedActor :type "Actor Object Reference"))
  (`self.K2_DestroyActor` DeletedActor))

(event `self.ReceiveBeginPlay`
  (bind _outactors (`GameplayStatics.GetAllActorsOfClass` "/Game/BhandanaDesign/VariableData/BP_GlobalVariables.BP_GlobalVariables_C"))
  (set `self.DamageTypes` (`/Game/BhandanaDesign/VariableData/BP_GlobalVariables.DamageTypes` (`|GetArrayItem` _outactors))))

(fn `UserConstructionScript`)