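; Explosive barrel that loses health from any damage and, at zero, waits briefly, deals radial damage with falloff once, then destroys itself.
; Its DamageType sets both the blast's damage class and the material glow color in the construction script.
; Editor events flip the material's rotation direction and debug-draw the blast radius with lines to overlapping dynamic actors.
; GetEnemyData reports its name, health and faction.
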(event `self.ReceiveAnyDamage`
  (params (Damage :type "Float (single-precision)") (DamageType :type "DamageType Object Reference") (InstigatedBy :type "Controller Object Reference") (DamageCauser :type "Actor Object Reference"))
  (bind _damage (`self.Damage`))
  (bind _blast_radius (`self.Blast Radius`))
  (bind _output_get (set `self.Health` (- (`self.Health`) (`KismetMathLibrary.Round` Damage))))
  (if (<= _output_get 0)
    (`/Engine/EditorBlueprintResources/StandardMacros.DoOnce` false
      (:`Completed`
        (`KismetSystemLibrary.Delay` 0.5)
        (`GameplayStatics.ApplyRadialDamageWithFalloff` (`KismetMathLibrary.Conv_IntToDouble` _damage) (`KismetMathLibrary.Conv_IntToDouble` (/ _damage 2)) (`self.K2_GetActorLocation`) (/ _blast_radius 2.0) _blast_radius 1.0 (`/Game/BhandanaDesign/Actors/OBJ_CustomMacros.Get DamageType` (`self.Damage Type`)) (`|MakeArray` self :!type "Actor Object Reference") null null)
        (`self.K2_DestroyActor`)))))

(event `Change Rotation`
  ;[1 1 1] Changes the Direction the Barrel rotates
  (`/Engine/EditorBlueprintResources/StandardMacros.FlipFlop`
    (:`A`
      (set `self.RotationSpeed` -0.1))
    (:`B`
      (set `self.RotationSpeed` 0.1)))
  (`MeshComponent.SetScalarParameterValueOnMaterials` (`self.Model`) "Rotation Speed" (`self.RotationSpeed`)))

(event `Check Blast Radius`
  (bind _blast_radius (`self.Blast Radius`))
  (bind _returnvalue (`SceneComponent.K2_GetComponentLocation` (`self.Model`)))
  ;[1 1 1] Checks and displays all objects that would react to an explosion, as well as the explosion's size
  (`KismetSystemLibrary.SphereTraceSingle` :`Start` _returnvalue :`End` _returnvalue :`Radius` _blast_radius :`TraceChannel` "TraceTypeQuery1" :`DrawDebugType` "ForDuration" :`TraceColor` (struct :`G` 1.0 :`B` 0.139189 :`A` 1.0))
  (bind _outactors (`KismetSystemLibrary.SphereOverlapActors` _returnvalue _blast_radius (`|MakeArray` "ObjectTypeQuery2" :!type "EObjectTypeQuery Enum") null (`|MakeArray` self :!type "Actor Object Reference")))
  (for _array_element _outactors
    (bind _origin (`self.GetActorBounds` _array_element false false))
    (`KismetSystemLibrary.LineTraceSingle` :`Start` (`self.GetActorBounds` false) :`End` _origin :`TraceChannel` "TraceTypeQuery4" :`DrawDebugType` "ForDuration" :`TraceHitColor` (struct :`R` 1.0 :`B` 0.022203 :`A` 1.0))
    (`KismetSystemLibrary.DrawDebugPoint` _origin 10.0 (struct :`R` 1.0 :`A` 1.0) 5.0)))

(fn `GetEnemyData`
  (params (`Tag Data` :type Name))
  (returns (Name :type String) (Level :type Integer) (Health :type Integer) (`Max Health` :type Integer) (`Faction Tag` :type "/Game/BhandanaDesign/VariableData/Enums/TeamFaction Enum"))
  (return "Explosive Barrel" 0 (`self.Health`) (`self.MaxHealth`) "NewEnumerator2"))

(fn `UserConstructionScript`
  (bind _model (`self.Model`))
  (`MeshComponent.SetVectorParameterValueOnMaterials` _model "GlowColor" (`KismetMathLibrary.Conv_LinearColorToVector` (`/Game/BhandanaDesign/Actors/OBJ_CustomMacros.Damage Type to Color` (`self.Damage Type`))))
  (`MeshComponent.SetScalarParameterValueOnMaterials` _model "Rotation Speed" (`self.RotationSpeed`)))