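; Spline-based road tool that builds a continuous road along an editable spline from a repeated static mesh.
; The Construction Script steps along the spline by a set Distance and adds a collision-enabled spline mesh component for each segment.
; Each segment's ends take the spline's local location and direction, scaled by a Tangent value to bend the mesh along the curve.
; The event graph holds no active logic.
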(fn `UserConstructionScript`
  (bind _spline (`self.Spline`))
  (bind _distance (`self.Distance`))
  (for _index (range (+ (`.ReturnValue` (`KismetMathLibrary.FMod` (`SplineComponent.GetSplineLength` (`self.Spline`)) (`self.Distance`))) 1))
    (bind _returnvalue (`AddComponent|NODE_AddSplineMeshComponent-0`))
    (`PrimitiveComponent.SetCollisionEnabled` _returnvalue "QueryAndPhysics")
    (`StaticMeshComponent.SetStaticMesh` _returnvalue (`self.Mesh`))
    (bind _returnvalue_2 (* _index _distance))
    (bind _returnvalue_3 (+ _returnvalue_2 _distance))
    (`SplineMeshComponent.SetStartAndEnd` _returnvalue (`SplineComponent.GetLocationAtDistanceAlongSpline` _spline _returnvalue_2 "Local") (* (`SplineComponent.GetDirectionAtDistanceAlongSpline` _spline _returnvalue_2 "Local") (`self.Tangent`)) (`SplineComponent.GetLocationAtDistanceAlongSpline` _spline _returnvalue_3 "Local") (* (`SplineComponent.GetDirectionAtDistanceAlongSpline` _spline _returnvalue_3 "Local") (`self.Tangent`)) true)))