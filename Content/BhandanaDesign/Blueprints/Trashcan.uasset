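; Trashcan is an interactable quest object that updates the quest message to "Find Evidence" when inspected.
; ReadyToInspect mirrors IsActivated, copied at BeginPlay through SelfEvent and again in the IsActivated OnRep function.
; Interact checks that flag, then passes a DoOnce so the Game State quest message update fires only once.
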(event `self.ReceiveBeginPlay`
  (`self.SelfEvent`))

(event `/Game/Blueprints/Interface/INT_Interact.Interact`
  (if (`self.Ready to Inspect`)
    (`/Engine/EditorBlueprintResources/StandardMacros.DoOnce` false
      (:`Completed`
        (message `/Game/BhandanaDesign/Interfaces/BPI_QuestSystem.UpdateQuests` (`GameplayStatics.GetGameState`) "Find Evidence")))))

(event `SelfEvent`
  (set `self.Ready to Inspect` (`self.isActivated`)))

(fn `OnRep_isActivated`
  (set `self.Ready to Inspect` (`self.isActivated`)))

(fn `UserConstructionScript`)