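; Work-in-progress editor scatter tool that places randomly positioned copies of a chosen mesh as instanced static meshes.
; The construction script rebuilds instances from saved transforms, so the layout persists across reruns.
; Toggling GenerateObjects acts as a one-shot button that clears them and rerolls placements on a second new component.
; New transforms use random X/Y offsets scaled by a scatter distance, plus random yaw.
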(fn `Generate_Placements`
  (bind (_returnvalue_roll _returnvalue_pitch _returnvalue_yaw) (`KismetMathLibrary.BreakRotator` (`KismetMathLibrary.RandomRotator` false)))
  (`KismetArrayLibrary.Array_Clear` (`self.MEMORY_Transforms`))
  (bind _returnvalue (`AddComponent|NODE_AddInstancedStaticMeshComponent-0`))
  (`StaticMeshComponent.SetStaticMesh` _returnvalue (`self.Object Mesh`))
  (for _ (range 1 (+ (`self.Number of Objects`) 1))
    (bind _output_get (set `self.Mutual Transform` (`KismetMathLibrary.MakeTransform` (`KismetMathLibrary.MakeVector` (.x (* (`KismetMathLibrary.RandomUnitVector`) (`self.Scattering Distance`))) (.y (* (`KismetMathLibrary.RandomUnitVector`) (`self.Scattering Distance`)))) (`KismetMathLibrary.MakeRotator` 0.0 0.0 _returnvalue_yaw))))
    (`KismetArrayLibrary.Array_AddUnique` (`self.MEMORY_Transforms`) _output_get)
    (`InstancedStaticMeshComponent.AddInstance` _returnvalue _output_get)))

(fn `UserConstructionScript`
  (bind _returnvalue (`AddComponent|NODE_AddInstancedStaticMeshComponent-1`))
  (bind _output_get (set `self.ISMC_Ref` _returnvalue))
  (`StaticMeshComponent.SetStaticMesh` _output_get (`self.Object Mesh`))
  (for _array_element (`self.MEMORY_Transforms`)
    (`InstancedStaticMeshComponent.AddInstance` (`self.ISMC_Ref`) _array_element))
  (if (`self.Generate Objects`)
    (`InstancedStaticMeshComponent.ClearInstances` (`self.ISMC_Ref`))
    (set `self.Generate Objects` false)
    (`self.Generate_Placements`)))