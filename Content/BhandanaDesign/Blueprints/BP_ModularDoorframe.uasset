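; Modular doorframe wall piece with a physics door on a hinge constraint that reacts to damage.
; Point or weaker radial hits shove the door and briefly flip the hinge's angular target before resetting it.
; Strong radial damage destroys the hinge, blasts the door off with damage-scaled force, then removes it and sends a quest update.
; Construction builds the frame's dynamic material, and ConfigureDoor applies door mesh and room colors.
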(event `Blast Door Off`
  (params (Normal :type "Vector Structure") (Damage :type "Float (double-precision)"))
  (bind _door (`self.Door`))
  ;[1 1 1] Explodes the door off the wall -- The blast force is scaled off of damage
  (`PrimitiveComponent.AddImpulse` _door (* Normal (* Damage -500.0)) "None" false)
  (`PrimitiveComponent.SetAllPhysicsAngularVelocityInDegrees` _door (0.0 0.0 500.0) false)
  (`KismetSystemLibrary.Delay` 10.0)
  (`ActorComponent.K2_DestroyComponent` (`self.Door`))
  (message `/Game/BhandanaDesign/Interfaces/BPI_QuestSystem.UpdateQuests` (`GameplayStatics.GetGameState`) "BlowUpDoor"))

(event `self.ReceiveRadialDamage`
  (params (DamageReceived :type "Float (single-precision)") (DamageType :type "DamageType Object Reference") (Origin :type "Vector Structure") (HitInfo :type "HitResult Structure (by ref)") (InstigatedBy :type "Controller Object Reference") (DamageCauser :type "Actor Object Reference"))
  (if (>= DamageReceived 100.0)
    (`ActorComponent.K2_DestroyComponent` (`self.DoorwayHinge`))
    (`self.Blast Door Off` HitInfo_ImpactNormal DamageReceived)
    (else
      (`self.Multicast Impulse` HitInfo_ImpactNormal))))

(event `Multicast Impulse`
  (params (`Hit Normal` :type "Vector Structure"))
  (bind _returnvalue (* `Hit Normal` -1000.0))
  (bind _doorwayhinge (`self.DoorwayHinge`))
  (`PrimitiveComponent.AddImpulse` (`self.Door`) _returnvalue "None" true)
  (`PhysicsConstraintComponent.SetAngularOrientationTarget` _doorwayhinge (`KismetMathLibrary.MakeRotator` (select `bool` (> (.x _returnvalue) 0.0) :`false` -180.0 :`true` 180.0 :!type "Float (single-precision)")))
  (`KismetSystemLibrary.PrintString` "Off")
  (`KismetSystemLibrary.Delay` 2.5)
  (`PhysicsConstraintComponent.SetAngularOrientationTarget` _doorwayhinge (`KismetMathLibrary.MakeRotator` 0.0))
  (`KismetSystemLibrary.PrintString` "On")
  (`PrimitiveComponent.AddImpulse` (`self.Door`) (0.0 0.0 0.0) "None" false))

(event `self.ReceivePointDamage`
  (params (Damage :type "Float (single-precision)") (DamageType :type "DamageType Object Reference") (HitLocation :type "Vector Structure") (HitNormal :type "Vector Structure") (HitComponent :type "PrimitiveComponent Object Reference") (BoneName :type Name) (ShotFromDirection :type "Vector Structure") (InstigatedBy :type "Controller Object Reference") (DamageCauser :type "Actor Object Reference") (HitInfo :type "HitResult Structure (by ref)"))
  (`self.Multicast Impulse` HitNormal))

(event `ConfigureDoor`
  (params (`Room Data` :type "/Game/BhandanaDesign/VariableData/Structs/ModularHomes/ST_RoomData Structure"))
  (bind (_wallheight _wallmesh _roomtobuildoffof _wallindextobuildoffof _walldata _drawfloor _wallcolor _wall2color _trimcolor) (break `/Game/BhandanaDesign/VariableData/Structs/ModularHomes/ST_RoomData` `Room Data`))
  (bind _model (`self.Model`))
  (bind _door (`self.Door`))
  (bind (_roomindex _wallindex _islocked_ _doorcolor _doormodel) (break `/Game/BhandanaDesign/VariableData/Structs/ModularHomes/ST_DoorSettings` (`self.Door Settings`)))
  (`StaticMeshComponent.SetStaticMesh` _door _doormodel)
  (`MeshComponent.SetVectorParameterValueOnMaterials` _door "Door Color" (`KismetMathLibrary.Conv_LinearColorToVector` _doorcolor))
  (`MeshComponent.SetVectorParameterValueOnMaterials` _model "WallColor" (`KismetMathLibrary.Conv_LinearColorToVector` _wallcolor))
  (`MeshComponent.SetVectorParameterValueOnMaterials` _model "TrimColor" (`KismetMathLibrary.Conv_LinearColorToVector` _trimcolor))
  (`MeshComponent.SetVectorParameterValueOnMaterials` _model "WallColor2" (`KismetMathLibrary.Conv_LinearColorToVector` (select `bool` false :`false` _wallcolor :`true` _wall2color))))

(event `self.ReceiveBeginPlay`)

(fn `UserConstructionScript`
  (bind _returnvalue (`PrimitiveComponent.CreateDynamicMaterialInstance` (`self.Model`) 0 "/Game/BhandanaDesign/Textures/ModularHomes/Doorway1/ModularHouseINST.ModularHouseINST" "None"))
  (`MaterialInstanceDynamic.SetTextureParameterValue` _returnvalue "UVImage" "/Game/BhandanaDesign/Textures/ModularHomes/Doorway1/Door1MaskImgChannels_Base_Color.Door1MaskImgChannels_Base_Color")
  (`MaterialInstanceDynamic.SetTextureParameterValue` _returnvalue "HeightMap" "/Game/BhandanaDesign/Textures/ModularHomes/Doorway1/Wall1Height_Height.Wall1Height_Height")
  (`MaterialInstanceDynamic.SetTextureParameterValue` _returnvalue "NormalMap" "/Game/BhandanaDesign/Textures/ModularHomes/Doorway1/Wall1Height_Normal.Wall1Height_Normal")
  (cast `/Game/BhandanaDesign/Blueprints/BP_ModularWall` (`self.GetParentActor`)))