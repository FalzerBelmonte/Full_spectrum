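; ArrowStormHandler is an actor that spawns waves of downward arrow projectiles for an arrow storm attack.
; FireWave spawns randomly scattered arrows within BlastRadius-scaled X/Y values, without adding the actor's location, plus one above each supplied target.
; All arrows spawn at the actor's height with the passed damage, normal damage type and "Enemy" tag.
; CheckBlastRadius draws a debug circle of the radius around the actor.
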(event `Check Blast Radius`
  (`KismetSystemLibrary.DrawDebugCircle` (`self.K2_GetActorLocation`) (`self.Blast Radius`) 35 (struct :`R` 1.0 :`G` 0.008603 :`A` 1.0) 5.0 5.0 (-1.0 1.0 0.0) (1.0 1.0 0.0)))

(event `Fire Wave`
  (params (Quantity :type Integer) (Targets :type "Array of Actor Object Reference") (Damage :type Integer))
  (bind (_returnvalue_x _returnvalue_y _returnvalue_z) (`KismetMathLibrary.BreakVector` (`self.K2_GetActorLocation`)))
  (bind (_returnvalue_x_2 _returnvalue_y_2 _returnvalue_z_2) (`KismetMathLibrary.BreakVector` (`self.K2_GetActorLocation`)))
  (bind (_returnvalue_x_3 _returnvalue_y_3) (`KismetMathLibrary.BreakVector` (* (`KismetMathLibrary.Normal` (`KismetMathLibrary.MakeVector` (`KismetMathLibrary.RandomFloatInRange` -1.0 1.0) (`KismetMathLibrary.RandomFloatInRange` -1.0 1.0))) (`KismetMathLibrary.RandomFloatInRange` 0.0 (`self.Blast Radius`)))))
  (for _ (range (+ Quantity 1))
    (`|SpawnActorFromClass` "/Game/BhandanaDesign/Actors/Projectiles/BP_Projectile_Arrow.BP_Projectile_Arrow_C" (`KismetMathLibrary.MakeTransform` (`KismetMathLibrary.MakeVector` _returnvalue_x_3 _returnvalue_y_3 _returnvalue_z) (struct :`Pitch` -90.0)) "Undefined" "OverrideRootScale" null "Enemy" Damage "/Game/BhandanaDesign/Widgets/BP_NormalDamage.BP_NormalDamage_C" (0.0 0.0 0.0) null))
  (for _array_element Targets
    (bind (_returnvalue_x_4 _returnvalue_y_4) (`KismetMathLibrary.BreakVector` (`self.K2_GetActorLocation` _array_element)))
    (`|SpawnActorFromClass` "/Game/BhandanaDesign/Actors/Projectiles/BP_Projectile_Arrow.BP_Projectile_Arrow_C" (`KismetMathLibrary.MakeTransform` (`KismetMathLibrary.MakeVector` _returnvalue_x_4 _returnvalue_y_4 _returnvalue_z_2) (struct :`Pitch` -90.0)) "Undefined" "OverrideRootScale" null "Enemy" Damage "/Game/BhandanaDesign/Widgets/BP_NormalDamage.BP_NormalDamage_C" (0.0 0.0 0.0) null)))

(fn `UserConstructionScript`)