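; Physics object actor that gets knocked and spun when a BP_Projectile overlaps it; despite the name, it contains no destruction logic.
; The Model component's begin-overlap event casts the other actor to BP_Projectile and scales the sweep's impact normal by that projectile's ImpulseStrength.
; That vector drives both a linear and an angular impulse on Model, with Model wired twice as the angular impulse target.
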(event `self.Model.OnComponentBeginOverlap`
  (params (OverlappedComponent :type "PrimitiveComponent Object Reference") (OtherActor :type "Actor Object Reference") (OtherComp :type "PrimitiveComponent Object Reference") (OtherBodyIndex :type Integer) (bFromSweep :type Boolean) (SweepResult :type "HitResult Structure (by ref)"))
  (bind _asbp_projectile (cast `/Game/BhandanaDesign/Actors/Projectiles/BP_Projectile` OtherActor))
  (bind _returnvalue (* (`.ImpactNormal` (`GameplayStatics.BreakHitResult` SweepResult)) (`/Game/BhandanaDesign/Actors/Projectiles/BP_Projectile.impulseStrength` _asbp_projectile)))
  (`PrimitiveComponent.AddImpulse` (`self.Model`) _returnvalue "None" false)
  (`PrimitiveComponent.AddAngularImpulseInDegrees` (`self.Model`) _returnvalue "None" false)
  (`PrimitiveComponent.AddAngularImpulseInDegrees` (`self.Model`) _returnvalue "None" false))

(fn `UserConstructionScript`
  (`parent.UserConstructionScript`))