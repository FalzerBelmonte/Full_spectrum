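; Modular building actor that generates rooms, doorframes, furniture and lights in its construction script from data arrays.
; Each room gets an instanced static mesh with a tinted dynamic material, chaining wall units from a chosen wall of another room.
; Doors replace wall instances with configured BP_ModularDoorframe child actors; FloorBuilder is empty.
; Separate events draw debug traces and experiment with a procedural mesh from recorded wall-top vertices.
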(event `GetRoomOrigins`
  (for _array_element (`self.MEMORY_ISMA`)
    (`KismetSystemLibrary.SphereTraceSingle` :`Start` (`KismetSystemLibrary.GetComponentBounds` _array_element) :`End` (`self.GetActorBounds` false) :`Radius` 25.0 :`TraceChannel` "TraceTypeQuery1" :`DrawDebugType` "ForDuration" :`DrawTime` 10.0)))

(event `self.ReceiveBeginPlay`)

(event `get Actor Bounds`
  (bind _memory_verticies (`self.MEMORY_Verticies`))
  (bind _returnvalue (- (`KismetArrayLibrary.Array_Length` _memory_verticies) 1))
  (bind _output (`|GetArrayItem` _memory_verticies _returnvalue))
  (`KismetSystemLibrary.PrintString` (`KismetStringLibrary.Conv_IntToString` _returnvalue) true true (struct :`R` 1.0 :`B` 0.786115 :`A` 1.0))
  (`KismetSystemLibrary.SphereTraceSingle` :`Start` _output :`End` _output :`Radius` 50.0 :`TraceChannel` "TraceTypeQuery1" :`DrawDebugType` "ForDuration" :`bIgnoreSelf` false :`DrawTime` 25.0))

(event `CustomEvent_0`)

(event `Draw Walls`
  (bind _origin (`self.GetActorBounds` false true))
  (bind _memory_verticies (`self.MEMORY_Verticies`))
  (bind _returnvalue (`AddComponent|NODE_AddProceduralMeshComponent-3`))
  (`KismetArrayLibrary.Array_AddUnique` _memory_verticies (`KismetMathLibrary.MakeVector` (.x _origin) (.y _origin) (* 2 250.0)))
  (`KismetArrayLibrary.Array_Clear` (`self.MEMORY_Triangles`))
  (`KismetArrayLibrary.Array_Clear` (`self.MEMORY_UVS`))
  (for (_ _array_index) _memory_verticies
    (`KismetArrayLibrary.Array_Append` (`self.MEMORY_Triangles`) (`|MakeArray` (- (`KismetArrayLibrary.Array_Length` _memory_verticies) 1) _array_index (+ _array_index 1)))
    (`KismetSystemLibrary.PrintString` (`KismetStringLibrary.Concat_StrStr` (`KismetStringLibrary.Conv_IntToString` 0) "  " (`KismetStringLibrary.Conv_IntToString` 0) "  " (`KismetStringLibrary.Conv_IntToString` 0))))
  (`PrimitiveComponent.SetMaterial` _returnvalue 0 "/Game/BhandanaDesign/Textures/ModularHomes/Doorway1/Modular_Simple_RGB_INST.Modular_Simple_RGB_INST")
  (`ProceduralMeshComponent.CreateMeshSection_LinearColor` :`self` _returnvalue :`Vertices` _memory_verticies :`Triangles` (`self.MEMORY_Triangles`) :`bCreateCollision` true))

(event `Check Verticies`
  (for _array_element (`self.MEMORY_Verticies`)
    (`KismetSystemLibrary.SphereTraceSingle` :`Start` _array_element :`End` _array_element :`Radius` 75.0 :`TraceChannel` "TraceTypeQuery1" :`DrawDebugType` "ForDuration")))

(fn `DoorBuilder`
  (for _array_element (`self.Door Index`)
    (bind (_roomindex _wallindex) (break `/Game/BhandanaDesign/VariableData/Structs/ModularHomes/ST_DoorSettings` _array_element))
    (bind _output (`|GetArrayItem` (`self.MEMORY_ISMA`) _roomindex))
    (bind _returnvalue (`AddComponent|NODE_AddChildActorComponent-1` :`RelativeTransform` (`InstancedStaticMeshComponent.GetInstanceTransform` _output _wallindex false)))
    (`ChildActorComponent.SetChildActorClass` _returnvalue "/Game/BhandanaDesign/Blueprints/BP_ModularDoorframe.BP_ModularDoorframe_C")
    (`InstancedStaticMeshComponent.RemoveInstance` _output _wallindex)
    (bind _asbp_modular_doorframe (cast `/Game/BhandanaDesign/Blueprints/BP_ModularDoorframe` (`ChildActorComponent.ChildActor` _returnvalue)))
    (set `/Game/BhandanaDesign/Blueprints/BP_ModularDoorframe.Room Settings` (`|GetArrayItem` (`self.Room Data`) _roomindex) _asbp_modular_doorframe)
    (set `/Game/BhandanaDesign/Blueprints/BP_ModularDoorframe.Door Settings` _array_element _asbp_modular_doorframe)
    (`/Game/BhandanaDesign/Blueprints/BP_ModularDoorframe.Multicast_ConfigureDoor` _asbp_modular_doorframe)))

(fn `FloorBuilder`)

(fn `FurnitureBuilder`
  (for _array_element (`self.Furniture Settings`)
    (bind _returnvalue (`AddComponent|NODE_AddInstancedStaticMeshComponent-3`))
    (bind (_mesh _transforms) (break `/Game/BhandanaDesign/VariableData/Structs/ModularHomes/ST_Furnitures` _array_element))
    (`StaticMeshComponent.SetStaticMesh` _returnvalue _mesh)
    (for _array_element_2 _transforms
      (`InstancedStaticMeshComponent.AddInstance` _returnvalue _array_element_2))))

(fn `LightBuilder`
  (for _array_element (`self.Spotlights`)
    (bind (_transform _intensity _color _attenuationradius _innerconeangle _outerconeangle) (break `/Game/BhandanaDesign/VariableData/Structs/ModularHomes/ST_LightSettings` _array_element))
    (bind _returnvalue (`AddComponent|NODE_AddSpotLightComponent-0` :`RelativeTransform` _transform))
    (`LightComponent.SetIntensity` _returnvalue _intensity)
    (`LightComponent.SetLightColor` _returnvalue (`KismetMathLibrary.Conv_ColorToLinearColor` _color) true)
    (`SpotLightComponent.SetOuterConeAngle` _returnvalue _outerconeangle)
    (`SpotLightComponent.SetInnerConeAngle` _returnvalue _innerconeangle)
    (`LocalLightComponent.SetAttenuationRadius` _returnvalue _attenuationradius))
  (for _array_element_2 (`self.Pointlights`)
    (bind (_transform_2 _intensity_2 _color_2 _attenuationradius_2) (break `/Game/BhandanaDesign/VariableData/Structs/ModularHomes/ST_PointLightSettings` _array_element_2))
    (bind _returnvalue_2 (`AddComponent|NODE_AddPointLightComponent-0` :`RelativeTransform` _transform_2))
    (`LightComponent.SetIntensity` _returnvalue_2 _intensity_2)
    (`LightComponent.SetLightColor` _returnvalue_2 (`KismetMathLibrary.Conv_ColorToLinearColor` _color_2) true)
    (`LocalLightComponent.SetAttenuationRadius` _returnvalue_2 _attenuationradius_2)))

(fn `UserConstructionScript`
  (`self.Wall Builder`)
  (`self.FloorBuilder`)
  (`self.DoorBuilder`)
  (`self.FurnitureBuilder`)
  (`self.LightBuilder`))

(fn `Wall Builder`
  (bind _memory_isma (`self.MEMORY_ISMA`))
  (`KismetArrayLibrary.Array_Clear` (`self.MEMORY_Verticies`))
  (for (_array_element _array_index) (`self.Room Data`)
    (bind _returnvalue (`AddComponent|NODE_AddInstancedStaticMeshComponent-0`))
    (`ActorComponent.SetIsReplicated` _returnvalue true)
    (bind _returnvalue_2 (`KismetArrayLibrary.Array_AddUnique` _memory_isma _returnvalue))
    (bind ((`WallHeight_2_AB9588D54C2EC000435976BC19BB9845` _wallheight) (`StartingHeight_34_060348CC4A7B72F7CCE73E8F216C4E8B` _startingheight) (`WallMesh_27_55A4161A42B9544DA05036A5C06AB141` _wallmesh) (`Texture_40_C8B5C13348C92A18CE4CA5A83F5D8B82` _texture) (`XTiling_47_EE5F359B42800E1177DCB295A878DDA7` _xtiling) (`Roomtobuildoffof_22_9CB79CA34BD6F259769C3E8020DA8277` _roomtobuildoffof) (`WallIndextobuildoffof_24_04975D704178E73693CF3C9DBB37EDA6` _wallindextobuildoffof) (`WallData_6_9C5D06B447ADE7C97D7C268A0839BD16` _walldata) (`Color1_35_520C3CE44228F05734F1EB9D34E40E50` _color1) (`Color2_36_0FF2EF78491F1D6FCF60D0ADD999D95F` _color2) (`Color3_37_593754C24104E977B1F7A9980983D11C` _color3) (`HideDraw_49_34B7443A49A1199343E9959BD313F22C` _hidedraw)) (break `/Game/BhandanaDesign/VariableData/Structs/ModularHomes/ST_RoomData` _array_element))
    (`StaticMeshComponent.SetStaticMesh` _returnvalue _wallmesh)
    (`self.ConfigureDynamicMaterial` _array_element _returnvalue_2
      (:`  `
        (set `self.MEMORY_Transform` (`InstancedStaticMeshComponent.GetInstanceTransform` (`|GetArrayItem` _memory_isma _roomtobuildoffof) _wallindextobuildoffof false))
        (for _index (range _wallheight)
          (for (_array_element_2 _array_index_2) _walldata
            (bind (_numberofunits _directionofwalls _rotationofwalls) (break `/Game/BhandanaDesign/VariableData/Structs/ModularHomes/ST_WallData` _array_element_2))
            (for _index_2 (range _numberofunits)
              (`self.SpawnWall` _array_index_2 _rotationofwalls _directionofwalls _index_2 _index _returnvalue_2 _startingheight (+ _wallheight _startingheight)))
            (set `self.MEMORY_Direction` _directionofwalls)))
        (if _hidedraw
          (`SceneComponent.SetVisibility` (`|GetArrayItem` (`self.MEMORY_ISMA`) _array_index) false false))))))