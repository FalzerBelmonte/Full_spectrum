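; Lootable chest actor that opens once on interaction and drops a randomly rolled weapon.
; Setting IsOpen triggers a rep notify that plays the model's animation; after a short delay it spawns a weapon drop rolled from LootTable and sends a "Chest" quest update to the game state.
; One-time chests register their display name with the game instance, which BeginPlay checks to restore the open state.
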(event `self.ReceiveBeginPlay`
  (bind _is_new (message `/Game/BhandanaDesign/Interfaces/BPI_FS_LevelSystem.Check if first time` (`GameplayStatics.GetGameInstance`) (`KismetSystemLibrary.GetDisplayName` self)))
  (set `self.isOpen` (not _is_new)))

(event `/Game/Blueprints/Interface/INT_Interact.Interact`
  (`/Engine/EditorBlueprintResources/StandardMacros.DoOnce` false
    (:`Completed`
      (set `self.isOpen` true)
      (`KismetSystemLibrary.Delay` 1.2)
      (bind _returnvalue (`|SpawnActorFromClass` "/Game/BhandanaDesign/Actors/Weapons/Weaponpickup/BP_WeaponDrop_MASTER.BP_WeaponDrop_MASTER_C" (`KismetMathLibrary.MakeTransform` (`self.GetActorBounds` false)) "Undefined" "OverrideRootScale" null null))
      (set `/Game/BhandanaDesign/Actors/Weapons/Weaponpickup/BP_WeaponDrop_MASTER.Weapon Data` (`/Game/BhandanaDesign/Actors/OBJ_CustomMacros.ROLL Random Weapon From Drop Table With Unique Stats` (`self.Loot Table`)) _returnvalue)
      (message `/Game/BhandanaDesign/Interfaces/BPI_QuestSystem.UpdateQuests` (`GameplayStatics.GetGameState`) "Chest")
      (if (`self.IsOneTimeOnly`)
        (message `/Game/BhandanaDesign/Interfaces/BPI_FS_LevelSystem.BPI_Add to Activated List` (`GameplayStatics.GetGameInstance`) (`KismetSystemLibrary.GetDisplayName` self))))))

(fn `BPI_Controller_GetLevelData`
  (returns (`Level Name` :type String))
  (return ""))

(fn `BPI_Get Level Map Name`
  (returns (`Level Name` :type String))
  (return ""))

(fn `BPI_Get Level Start Name`
  (returns (NewParam :type String))
  (return ""))

(fn `Check if first time`
  (params (`Actor to Check` :type String))
  (returns (`Is New` :type Boolean))
  (return false))

(fn `OnRep_Start Open`
  (if (`self.isOpen`)
    (`SkeletalMeshComponent.Play` (`self.Model`) false)))

(fn `Save Activated Tags`
  (returns (Tags :type "Array of String"))
  (return))

(fn `UserConstructionScript`)