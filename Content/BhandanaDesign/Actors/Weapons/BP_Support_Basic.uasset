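; BP_Support_Basic is a support weapon that fires healing projectiles.
; Attack triggers a multicast muzzle flash at the Barrel socket, then line traces on Visibility, ignoring its parent actor, to compute the projectile's rotation from the barrel.
; ServerSpawnBullet spawns P_HealingProjectile with a random amount between min and max damage, plus the weapon's damage type and tags.
; A separate point-damage event exists but is not called in this graph.
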(event `self.MULTICAST_MuzzleFlash`
  (bind _returnvalue (`SceneComponent.GetSocketTransform` (`self.Model`) "Barrel" "RTS_World"))
  ;[1 1 1] Handle the firing of a bullet and deals damage when it's supposed to
  (`GameplayStatics.SpawnEmitterAtLocation` "/Game/Materials/Muzzle_flash/Muzzle_flash.Muzzle_flash" (.location _returnvalue) (`KismetMathLibrary.MakeRotator` (.roll (.rotation _returnvalue)) (* (.pitch (.rotation _returnvalue)) -1.0) (+ (.yaw (.rotation _returnvalue)) 180.0)) (0.5 0.5 0.5)))

(event `self.SERVER_Muzzle Flash`
  ;[1 1 1] Handle the firing of a bullet and deals damage when it's supposed to
  (`self.MULTICAST_MuzzleFlash`))

(event `/Game/BhandanaDesign/Interfaces/BPI_FS_WeaponInteractions.Attack`
  (params (Weapon :type "/Game/BhandanaDesign/VariableData/Structs/ST_WeaponData Structure") (MinDamage :type Integer) (MaxDamage :type Integer) (RaycastStart :type "Vector Structure") (RaycastEnd :type "Vector Structure") (TagData :type Name) (`Camera Forward Vector` :type "Vector Structure"))
  ;[1 1 1] Handle the firing of a bullet and deals damage when it's supposed to
  (`self.MULTICAST_MuzzleFlash`)
  (bind (_outhit _returnvalue) (`KismetSystemLibrary.LineTraceSingle` RaycastStart RaycastEnd "TraceTypeQuery1" false (`|MakeArray` (`self.GetParentActor`) null)))
  (bind (_projetile_rotation _firepoint) (`/Game/BhandanaDesign/Actors/OBJ_CustomMacros.CalculateBulletPath` _outhit _returnvalue (`/Game/BhandanaDesign/Actors/OBJ_CustomMacros.Get Weapon Barrel` (`self.Model`)) Weapon TagData)
    (:`  `
      _)
    (:`Output with Hit`
      _))
  (`self.Server_Spawn Bullet` _firepoint _projetile_rotation))

(event `CustomEvent`
  (params (`Damaged Actor` :type "Actor Object Reference") (`base Damage` :type "Float (double-precision)") (`Hit From Direction` :type "Vector Structure") (`Hit Info` :type "HitResult Structure") (Instigator :type "Controller Object Reference") (Causer :type "Actor Object Reference") (`Damage Type` :type "DamageType Class Reference"))
  ;[1 1 1] Handle the firing of a bullet and deals damage when it's supposed to
  (`GameplayStatics.ApplyPointDamage` `Damaged Actor` `base Damage` `Hit From Direction` `Hit Info` Instigator self `Damage Type`))

(event `self.Server_Spawn Bullet`
  (params (`Spawn Location` :type "Vector Structure") (`Spawn Rotation` :type "Rotator Structure"))
  ;[1 1 1] Handle the firing of a bullet and deals damage when it's supposed to
  (`|SpawnActorFromClass` "/Game/BhandanaDesign/Actors/Projectiles/P_HealingProjectile.P_HealingProjectile_C" (`KismetMathLibrary.MakeTransform` `Spawn Location` `Spawn Rotation`) "Undefined" "OverrideRootScale" self (stale `/Game/BhandanaDesign/Interfaces/BPI_FS_WeaponInteractions.Attack` TagData) (`KismetMathLibrary.RandomIntegerInRange` (stale `/Game/BhandanaDesign/Interfaces/BPI_FS_WeaponInteractions.Attack` MinDamage) (stale `/Game/BhandanaDesign/Interfaces/BPI_FS_WeaponInteractions.Attack` MaxDamage)) (`.AsDamageType` (`/Game/BhandanaDesign/Actors/OBJ_CustomMacros.Get Weapon Damage Type` (stale `/Game/BhandanaDesign/Interfaces/BPI_FS_WeaponInteractions.Attack` Weapon))) (stale `/Game/BhandanaDesign/Interfaces/BPI_FS_WeaponInteractions.Attack` _firepoint) null))

(fn `UserConstructionScript`
  (`parent.UserConstructionScript`))