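; Master weapon actor that handles a weapon's appearance and hitscan attacks, with events relayed through server and multicast calls.
; UpdateVisuals sets the model's mesh, skin and damage-type glow color, then attaches to a skeletal mesh socket.
; Attack triggers a barrel muzzle flash and line traces while ignoring the parent actor.
; CalculateBulletPath decides whether the server call applies random point damage within the given range, typed by the weapon.
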(event `/Game/BhandanaDesign/Interfaces/BPI_FS_WeaponInteractions.UpdateVisuals`
  (params (Weapon :type "/Game/BhandanaDesign/VariableData/Structs/ST_WeaponData Structure") (`Sekletal Mesh` :type "SceneComponent Object Reference") (Socket :type Name))
  ;[1 1 1] This section handles visual appearance updates
  (`self.SERVER_Update Visuals` Weapon `Sekletal Mesh` Socket))

(event `MULTICAST_Update Visuals`
  (params (Weapon :type "/Game/BhandanaDesign/VariableData/Structs/ST_WeaponData Structure") (`Sekletal Mesh` :type "SceneComponent Object Reference") (Socket :type Name))
  (bind (_weapon_model _weapon_skin) (`/Game/BhandanaDesign/Actors/OBJ_CustomMacros.Get Weapon Model Visuals` Weapon))
  (bind _model (`self.Model`))
  ;[1 1 1] This section handles visual appearance updates
  (`StaticMeshComponent.SetStaticMesh` _model _weapon_model)
  (`PrimitiveComponent.SetMaterial` _model 0 _weapon_skin)
  (`MeshComponent.SetVectorParameterValueOnMaterials` _model "GlowColor" (`KismetMathLibrary.Conv_LinearColorToVector` (`/Game/BhandanaDesign/Actors/OBJ_CustomMacros.Damage Type to Color` (`/Game/BhandanaDesign/Actors/OBJ_CustomMacros.Get Weapon Damage Type` Weapon))))
  (`self.K2_AttachToComponent` `Sekletal Mesh` Socket "SnapToTarget" "SnapToTarget" "KeepRelative"))

(event `SERVER_Update Visuals`
  (params (Weapon :type "/Game/BhandanaDesign/VariableData/Structs/ST_WeaponData Structure") (`Sekletal Mesh` :type "SceneComponent Object Reference") (Socket :type Name))
  ;[1 1 1] This section handles visual appearance updates
  (`self.MULTICAST_Update Visuals` Weapon `Sekletal Mesh` Socket))

(event `MULTICAST_MuzzleFlash`
  (bind _returnvalue (`SceneComponent.GetSocketTransform` (`self.Model`) "Barrel" "RTS_World"))
  ;[1 1 1] Handle the firing of a bullet and deals damage when it's supposed to
  (`GameplayStatics.SpawnEmitterAtLocation` "/Game/Materials/Muzzle_flash/Muzzle_flash.Muzzle_flash" (.location _returnvalue) (`KismetMathLibrary.MakeRotator` (.roll (.rotation _returnvalue)) (* (.pitch (.rotation _returnvalue)) -1.0) (+ (.yaw (.rotation _returnvalue)) 180.0)) (0.5 0.5 0.5)))

(event `SERVER_Muzzle Flash`
  ;[1 1 1] Handle the firing of a bullet and deals damage when it's supposed to
  (`self.MULTICAST_MuzzleFlash`))

(event `/Game/BhandanaDesign/Interfaces/BPI_FS_WeaponInteractions.Attack`
  (params (Weapon :type "/Game/BhandanaDesign/VariableData/Structs/ST_WeaponData Structure") (MinDamage :type Integer) (MaxDamage :type Integer) (RaycastStart :type "Vector Structure") (RaycastEnd :type "Vector Structure") (TagData :type Name))
  ;[1 1 1] Handle the firing of a bullet and deals damage when it's supposed to
  (`self.SERVER_Muzzle Flash`)
  (bind (_outhit _returnvalue) (`KismetSystemLibrary.LineTraceSingle` RaycastStart RaycastEnd "TraceTypeQuery1" false (`|MakeArray` (`self.GetParentActor`))))
  (bind (_projetile_rotation _firepoint _should_i_do_damage_ _who_i_hit) (`/Game/BhandanaDesign/Actors/OBJ_CustomMacros.CalculateBulletPath` _outhit _returnvalue (`/Game/BhandanaDesign/Actors/OBJ_CustomMacros.Get Weapon Barrel` (`self.Model`)) Weapon TagData)
    (:`Output with Hit`
      (if _should_i_do_damage_
        (`self.SERVER_Point Damage` _who_i_hit (`KismetMathLibrary.Conv_IntToDouble` (`KismetMathLibrary.RandomIntegerInRange` MinDamage MaxDamage)) (0.0 0.0 0.0) _outhit (`GameplayStatics.GetPlayerController` 0) null (`.AsDamageType` (`/Game/BhandanaDesign/Actors/OBJ_CustomMacros.Get Weapon Damage Type` Weapon)))))))

(event `SERVER_Point Damage`
  (params (`Damaged Actor` :type "Actor Object Reference") (`base Damage` :type "Float (double-precision)") (`Hit From Direction` :type "Vector Structure") (`Hit Info` :type "HitResult Structure") (Instigator :type "Controller Object Reference") (Causer :type "Controller Object Reference") (`Damage Type` :type "DamageType Class Reference"))
  ;[1 1 1] Handle the firing of a bullet and deals damage when it's supposed to
  (`GameplayStatics.ApplyPointDamage` `Damaged Actor` `base Damage` `Hit From Direction` `Hit Info` Instigator self `Damage Type`))

(fn `UserConstructionScript`)