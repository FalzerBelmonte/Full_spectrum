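; BP_EnergyShield is a damageable energy shield that loses health when hit, shuts off when depleted and recharges after a delay.
; AnyDamage subtracts from the weapon data's shield stats, disabling the mesh at zero, and restarts the delay timer that re-enables it.
; The IsCharging RepNotify starts a self-rescheduling tick that increments health, with no clamp wired in.
; A dynamic material's HealthPercent parameter displays remaining health.
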(event `EnableShield`
  (bind _shieldmesh (`self.ShieldMesh`))
  (`ActorComponent.Activate` _shieldmesh false)
  (`PrimitiveComponent.SetCollisionEnabled` _shieldmesh "QueryOnly")
  (`SceneComponent.SetVisibility` _shieldmesh true false))

(event `RechargeTick`
  (bind _weapondata (`self.WeaponData`))
  (bind (_weapondata_weaponinformation _weapondata_weaponvisuals _weapondata_weaponstats _weapondata_projectileinformation _weapondata_shieldstats) (break `/Game/BhandanaDesign/VariableData/Structs/ST_WeaponData` (`self.WeaponData`)))
  (if (`self.isCharging`)
    (bind _result (`/Engine/EditorBlueprintResources/StandardMacros.IncrementInt` (`/Game/BhandanaDesign/Actors/OBJ_CustomMacros.Get Shield Health` _weapondata))
      (:`  `
        (bind _structout (setmembers `/Game/BhandanaDesign/VariableData/Structs/ST_ShieldData` :`StructRef` _weapondata_shieldstats))
        (set `self.WeaponData` (make `/Game/BhandanaDesign/VariableData/Structs/ST_WeaponData` _weapondata_weaponinformation _weapondata_weaponvisuals _weapondata_weaponstats _weapondata_projectileinformation _structout))
        (`self.UpdateShield`)
        (bind _returnvalue (`KismetSystemLibrary.K2_SetTimerDelegate` (delegate `RechargeTick`) (`.RechargeSpeed_7_3B2F8FBD45A6992665DE5FBA894F3237` (break `/Game/BhandanaDesign/VariableData/Structs/ST_ShieldData` (`.ShieldStats_85_E23A2CC641C9A943846F2E81E44B3E5D` (break `/Game/BhandanaDesign/VariableData/Structs/ST_WeaponData` _weapondata))))))))
    (else
      (`KismetSystemLibrary.K2_ClearAndInvalidateTimerHandle` _returnvalue))))

(event `BeginRecharge`
  (`self.EnableShield`)
  (set `self.isCharging` true))

(event `DisableShield`
  (bind _shieldmesh (`self.ShieldMesh`))
  (`ActorComponent.Deactivate` _shieldmesh)
  (`PrimitiveComponent.SetCollisionEnabled` _shieldmesh "NoCollision")
  (`SceneComponent.SetVisibility` _shieldmesh false false))

(event `UpdateShield`
  (bind _weapondata (`self.WeaponData`))
  (`MaterialInstanceDynamic.SetScalarParameterValue` (stale `self.ReceiveBeginPlay` _returnvalue) "HealthPercent" (/ (`KismetMathLibrary.Conv_IntToDouble` (`.ShieldHealth_13_7298EB114B75139F880AD79DDB27B9CE` (break `/Game/BhandanaDesign/VariableData/Structs/ST_ShieldData` (`.ShieldStats_85_E23A2CC641C9A943846F2E81E44B3E5D` (break `/Game/BhandanaDesign/VariableData/Structs/ST_WeaponData` _weapondata))))) (`KismetMathLibrary.Conv_IntToDouble` (`.ShieldHealthMax_15_B65913B74199E51E11C580AA12E2F41F` (break `/Game/BhandanaDesign/VariableData/Structs/ST_ShieldData` (`.ShieldStats_85_E23A2CC641C9A943846F2E81E44B3E5D` (break `/Game/BhandanaDesign/VariableData/Structs/ST_WeaponData` _weapondata)))))) :!label _label))

(event `self.ReceiveBeginPlay`
  (`parent.ReceiveBeginPlay`)
  (`self.Initalize` (`self.isStartEnabled`))
  (bind _output_get (set `self.ShieldData` (`PrimitiveComponent.GetMaterial` (`self.ShieldMesh`) 0)))
  (bind _returnvalue (`PrimitiveComponent.CreateDynamicMaterialInstance` (`self.ShieldMesh`) 0 _output_get "None"))
  (goto _label))

(event `self.ReceiveAnyDamage`
  (params (Damage :type "Float (single-precision)") (DamageType :type "DamageType Object Reference") (InstigatedBy :type "Controller Object Reference") (DamageCauser :type "Actor Object Reference"))
  (`self.HitShield`)
  (`self.DamageMacro` Damage))

(event `Initalize`
  (params (`start active` :type Boolean))
  (if (not `start active`)
    (`self.DisableShield`)))

(event `HitShield`
  (set `self.isCharging` false)
  (`KismetSystemLibrary.K2_SetTimerDelegate` (delegate `BeginRecharge`) (`.DelayBeforeRecharge_6_FC5430C64E4F627027433D9570A21A2F` (break `/Game/BhandanaDesign/VariableData/Structs/ST_ShieldData` (`.ShieldStats_85_E23A2CC641C9A943846F2E81E44B3E5D` (break `/Game/BhandanaDesign/VariableData/Structs/ST_WeaponData` (`self.WeaponData`)))))))

(fn `OnRep_isCharging`
  (`self.RechargeTick`))

(fn `UserConstructionScript`
  (`parent.UserConstructionScript`))