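; BP_EnergyShield1 is an energy shield weapon that raises its Shield component while aiming down sights.
; The multicast begin-ADS event calls the parent, assigns tags to the Shield, shows it and sets its HealthPercent material parameter to a fixed value.
; The end-ADS event hides the Shield without calling the parent; both events print a debug string.
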(event `self.Multicast_Begin ADS`
  (bind _shield (`self.Shield`))
  (`parent.Multicast_Begin ADS`)
  (set `ActorComponent.ComponentTags` (`self.Tag Data`) _shield)
  (`SceneComponent.SetVisibility` _shield true false)
  (`KismetSystemLibrary.PrintString` "Active")
  (`MeshComponent.SetScalarParameterValueOnMaterials` (`self.Shield`) "HealthPercent" 0.2)
  (`MeshComponent.SetScalarParameterValueOnMaterials` _shield "HealthPercent" 0.2))

(event `self.Multicast_End ADS`
  (`SceneComponent.SetVisibility` (`self.Shield`) false false)
  (`KismetSystemLibrary.PrintString` "Inactive"))

(fn `UserConstructionScript`
  (`parent.UserConstructionScript`))