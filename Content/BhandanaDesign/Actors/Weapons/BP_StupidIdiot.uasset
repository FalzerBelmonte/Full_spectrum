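; BP_StupidIdiot is a weapon visual actor that displays a weapon's model and plays audio while attacking.
; UpdateVisuals routes through a server event to a multicast, which sets the Model's mesh and skin from the weapon's data.
; The multicast also tints the GlowColor material parameter by damage type and snaps to the given skeletal mesh socket.
; BeginAttacking and StopAttacking start and stop the Audio component, with no RPC routing in this graph.
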(event `/Game/BhandanaDesign/Interfaces/BPI_FS_WeaponInteractions.UpdateVisuals`
  (params (Weapon :type "/Game/BhandanaDesign/VariableData/Structs/ST_WeaponData Structure") (`Sekletal Mesh` :type "SceneComponent Object Reference") (Socket :type Name))
  (`self.SERVER_Update Visuals` Weapon `Sekletal Mesh` Socket))

(event `MULTICAST_Update Visuals`
  (params (Weapon :type "/Game/BhandanaDesign/VariableData/Structs/ST_WeaponData Structure") (`Sekletal Mesh` :type "SceneComponent Object Reference") (Socket :type Name))
  (bind (_weapon_model _weapon_skin) (`/Game/BhandanaDesign/Actors/OBJ_CustomMacros.Get Weapon Model Visuals` Weapon))
  (bind _model (`self.Model`))
  (`StaticMeshComponent.SetStaticMesh` _model _weapon_model)
  (`PrimitiveComponent.SetMaterial` _model 0 _weapon_skin)
  (`MeshComponent.SetVectorParameterValueOnMaterials` _model "GlowColor" (`KismetMathLibrary.Conv_LinearColorToVector` (`/Game/BhandanaDesign/Actors/OBJ_CustomMacros.Damage Type to Color` (`/Game/BhandanaDesign/Actors/OBJ_CustomMacros.Get Weapon Damage Type` Weapon))))
  (`self.K2_AttachToComponent` `Sekletal Mesh` Socket "SnapToTarget" "SnapToTarget" "KeepRelative"))

(event `SERVER_Update Visuals`
  (params (Weapon :type "/Game/BhandanaDesign/VariableData/Structs/ST_WeaponData Structure") (`Sekletal Mesh` :type "SceneComponent Object Reference") (Socket :type Name))
  (`self.MULTICAST_Update Visuals` Weapon `Sekletal Mesh` Socket))

(event `/Game/BhandanaDesign/Interfaces/BPI_FS_WeaponInteractions.BeginAttacking`
  (`AudioComponent.Play` (`self.Audio`) 0.0))

(event `/Game/BhandanaDesign/Interfaces/BPI_FS_WeaponInteractions.StopAttacking`
  (`AudioComponent.Stop` (`self.Audio`)))

(fn `UserConstructionScript`)