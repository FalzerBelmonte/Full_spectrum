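; Gun Blueprint that raises a shield while aiming down sights.
; OnADS calls MulticastOnADS, which applies the current weapon's shield material to ShieldMesh and activates the shield through ShieldHandler.
; Ending ADS or unequipping goes through ServerADSEnd, which deactivates it with the same weapon data.
; The weapon's ShieldModel stat is read by an unconnected node, so the mesh itself is not swapped here.
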(event `self.OnUnequip`
  (`self.OnADSEnd`))

(event `Multicast OnADS`
  (`PrimitiveComponent.SetMaterial` (`self.Shield Mesh`) 0 (`.ShieldMaterial_20_6222712944305FCD56C3689F1A36B3EF` (break `/Game/BhandanaDesign/VariableData/Structs/ST_ShieldData` (`.ShieldStats_85_E23A2CC641C9A943846F2E81E44B3E5D` (break `/Game/BhandanaDesign/VariableData/Structs/ST_WeaponData` (`/Game/BhandanaDesign/Actors/RPG_Actor.CurrentWeapon` (`self.ParentActor`)))))))
  (`self.Shield Handler` true (`/Game/BhandanaDesign/Actors/RPG_Actor.CurrentWeapon` (`self.ParentActor`))))

(event `self.OnADS`
  (`self.Multicast OnADS`))

(event `self.OnADSEnd`
  (`self.Server ADS End`))

(event `Server ADS End`
  (`self.Shield Handler` false (`/Game/BhandanaDesign/Actors/RPG_Actor.CurrentWeapon` (`self.ParentActor`))))

(fn `UserConstructionScript`
  (`parent.UserConstructionScript`))