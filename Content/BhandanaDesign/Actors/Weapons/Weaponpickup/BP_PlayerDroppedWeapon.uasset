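; Weapon pickup Blueprint for a weapon dropped by the player, adding a physics-based toss to its parent class.
; Its LaunchObject event applies a mass-independent forward impulse to the Model component, then sets a random angular velocity on each axis so it tumbles.
; The construction script defers to the parent, and the overlap and tick events are unused disabled stubs.
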(event `self.LaunchObject`
  (`PrimitiveComponent.AddImpulse` (`self.Model`) (* (`self.GetActorForwardVector`) 450.0) "None" true)
  (`PrimitiveComponent.SetPhysicsAngularVelocityInDegrees` (`self.Model`) (`KismetMathLibrary.MakeVector` (`KismetMathLibrary.RandomFloatInRange` -500.0 500.0) (`KismetMathLibrary.RandomFloatInRange` -500.0 500.0) (`KismetMathLibrary.RandomFloatInRange` -500.0 500.0)) false "None"))

(fn `UserConstructionScript`
  (`parent.UserConstructionScript`))