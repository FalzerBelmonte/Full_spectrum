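; Master weapon drop actor that represents a loot pickup in the world, with a mesh and an info window driven by its WeaponData.
; VisualUpdate, also run from the construction script, sets mesh, skin and damage-type glow, fills the widget's stats, then launches the drop with random impulse and spin on authority.
; ToggleUIPanel shows or hides the window based on whether it is looked at.
; Cleanup removes the widget and destroys the actor.
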(event `Toggle UI Panel`
  (params (`Is Looked at` :type Boolean))
  (bind _my_widget (`self.my Widget`))
  (if `Is Looked at`
    (`/Engine/EditorBlueprintResources/StandardMacros.IsValid` _my_widget
      (:`Is Valid`
        (`UserWidget.AddToViewport` _my_widget 1)
        (`|PlayAnimation` _my_widget (`/Game/BhandanaDesign/Widgets/BP_PickupWindow.FadeIn` _my_widget)
          (:`Finished`
            (set `self.is In Viewport` true)))))
    (else
      (`/Engine/EditorBlueprintResources/StandardMacros.IsValid` _my_widget
        (:`Is Valid`
          (`Widget.RemoveFromParent` _my_widget))))))

(event `Server Visual Update`
  (`self.Visual Update`))

(event `Visual Update`
  (bind _model (`self.Model`))
  (bind _weapon_data (`self.Weapon Data`))
  (bind _my_widget (`self.my Widget`))
  (bind (_weapon_model _weapon_skin) (`/Game/BhandanaDesign/Actors/OBJ_CustomMacros.Get Weapon Model Visuals` (`self.Weapon Data`)))
  (bind (_name _description) (`/Game/BhandanaDesign/Actors/OBJ_CustomMacros.Get Weapon Name` _weapon_data))
  (bind (_min_damage _max_damage) (`/Game/BhandanaDesign/Actors/OBJ_CustomMacros.Get Weapon Damage` _weapon_data))
  (bind (_linear_weapon_color _slate_weapon_color) (`/Game/BhandanaDesign/Actors/OBJ_CustomMacros.Damage Type to Color` (`/Game/BhandanaDesign/Actors/OBJ_CustomMacros.Get Weapon Damage Type` _weapon_data)))
  (`StaticMeshComponent.SetStaticMesh` _model _weapon_model)
  (`PrimitiveComponent.SetMaterial` _model 0 _weapon_skin)
  (`/Engine/EditorBlueprintResources/StandardMacros.IsValid` _my_widget
    (:`Is Valid`
      (set `/Game/BhandanaDesign/Widgets/BP_PickupWindow.VAR_WeaponName` (`KismetStringLibrary.Conv_NameToString` _name) _my_widget)
      (set `/Game/BhandanaDesign/Widgets/BP_PickupWindow.VAR_WeaponDescription` (select `bool` (!= _description "None") :`true` (`KismetStringLibrary.Conv_NameToString` _description)) _my_widget)
      (set `/Game/BhandanaDesign/Widgets/BP_PickupWindow.VAR_DamageRange` (`KismetStringLibrary.Concat_StrStr` (`KismetStringLibrary.Conv_IntToString` _min_damage) " - " (`KismetStringLibrary.Conv_IntToString` _max_damage)) _my_widget)
      (set `/Game/BhandanaDesign/Widgets/BP_PickupWindow.VAR_ClipSize` (`KismetStringLibrary.Conv_IntToString` (`.Clip Size` (`/Game/BhandanaDesign/Actors/OBJ_CustomMacros.Get Weapon Ammo` _weapon_data))) _my_widget)
      (set `/Game/BhandanaDesign/Widgets/BP_PickupWindow.VAR_WeaponAccuracy` (`KismetStringLibrary.Concat_StrStr` (`KismetStringLibrary.Conv_IntToString` (`/Game/BhandanaDesign/Actors/OBJ_CustomMacros.Get Weapon Accuracy` _weapon_data)) "%") _my_widget)
      (set `/Game/BhandanaDesign/Widgets/BP_PickupWindow.VAR_WindowColor` _slate_weapon_color _my_widget)
      (`MeshComponent.SetVectorParameterValueOnMaterials` (`self.Model`) "GlowColor" (`KismetMathLibrary.Conv_LinearColorToVector` _linear_weapon_color))
      (set `/Game/BhandanaDesign/Widgets/BP_PickupWindow.VAR_FireRate` (`/Game/BhandanaDesign/Actors/OBJ_CustomMacros.LOOTUI_Firemode_and_Rate_to_String` (`/Game/BhandanaDesign/Actors/OBJ_CustomMacros.Get Weapon Fire Mode` _weapon_data) (`/Game/BhandanaDesign/Actors/OBJ_CustomMacros.Get Weapon Fire Rate` _weapon_data)) _my_widget)
      (`/Engine/EditorBlueprintResources/ActorMacros.Switch Has Authority`
        (:`Authority`
          (`self.LaunchObject`))))))

(event `self.ReceiveBeginPlay`
  (bind _returnvalue (`|CreateWidget` "/Game/BhandanaDesign/Widgets/BP_PickupWindow.BP_PickupWindow_C"))
  (set `self.my Widget` _returnvalue))

(event `Server_Cleanup`
  (`self.Cleanup`))

(event `Cleanup`
  (bind _my_widget (`self.my Widget`))
  (`/Engine/EditorBlueprintResources/StandardMacros.IsValid` _my_widget
    (:`Is Valid`
      (`Widget.RemoveFromParent` _my_widget)
      (`self.K2_DestroyActor`))))

(event `LaunchObject`
  (`PrimitiveComponent.AddImpulse` (`self.Model`) (`KismetMathLibrary.MakeVector` (`KismetMathLibrary.RandomFloatInRange` -150.0 150.0) (`KismetMathLibrary.RandomFloatInRange` -150.0 150.0) 500.0) "None" true)
  (`PrimitiveComponent.SetPhysicsAngularVelocityInDegrees` (`self.Model`) (`KismetMathLibrary.MakeVector` (`KismetMathLibrary.RandomFloatInRange` -500.0 500.0) (`KismetMathLibrary.RandomFloatInRange` -500.0 500.0) (`KismetMathLibrary.RandomFloatInRange` -500.0 500.0)) false "None"))

(fn `OnRep_Weapon Data`)

(fn `UserConstructionScript`
  (`self.Visual Update`))