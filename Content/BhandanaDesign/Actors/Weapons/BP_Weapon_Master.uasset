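; Base weapon actor attached to an RPG_Actor, with empty equip, ADS and special hooks and a built-in shield.
; BeginPlay applies the owner's CurrentWeapon visuals and shield setup, while equipping tints the glow by damage type.
; Attack routes to a server-named event that traces the aim line and spawns projectiles, assigning random damage, type and tag on authority.
; Damage drains shield health stored in CurrentWeapon, updates the material, disables depleted shields and triggers the owner's recharge.
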(event `OnEquip`
  (bind _parentactor (`self.ParentActor`))
  (`/Engine/EditorBlueprintResources/StandardMacros.IsValid` _parentactor
    (:`Is Valid`
      (`/Game/BhandanaDesign/Actors/RPG_Actor.Set Shield Recharge` _parentactor)
      (`self.ServerUpdateGlow` (`self.ParentActor`)))))

(event `ServerUpdateGlow`
  (params (`Parent Actor` :type "/Game/BhandanaDesign/Actors/RPG_Actor Object Reference"))
  (`MeshComponent.SetVectorParameterValueOnMaterials` (`self.Model`) "GlowColor" (`KismetMathLibrary.Conv_LinearColorToVector` (select `/Game/BhandanaDesign/VariableData/Enums/DamageTypes` (`/Game/BhandanaDesign/Actors/OBJ_CustomMacros.Get Weapon Damage Type` (`/Game/BhandanaDesign/Actors/RPG_Actor.CurrentWeapon` `Parent Actor`)) :`NewEnumerator0` (struct :`R` 1.0 :`G` 1.0 :`B` 1.0 :`A` 1.0) :`NewEnumerator1` (struct :`R` 1.0 :`A` 1.0) :`NewEnumerator2` (struct :`G` 0.848808 :`B` 1.0 :`A` 1.0) :!type "LinearColor Structure"))))

(event `OnADSEnd`)

(event `OnADS`)

(event `WeaponSpecial`)

(event `OnUnequip`)

(event `UpdateBulletProperties`
  (params (FinalDamage :type Integer) (DamageType :type "DamageType Class Reference") (Bullet :type "/Game/BhandanaDesign/Actors/Projectiles/BP_Projectile Object Reference") (tag :type Name))
  (set `/Game/BhandanaDesign/Actors/Projectiles/BP_Projectile.TagData` tag Bullet)
  (set `/Game/BhandanaDesign/Actors/Projectiles/BP_Projectile.Damage` FinalDamage Bullet)
  (set `/Game/BhandanaDesign/Actors/Projectiles/BP_Projectile.DamageType` DamageType Bullet))

(event `Attack`
  (params (Instigator :type "/Game/BhandanaDesign/Actors/RPG_Actor Object Reference") (OwnerTag :type Name) (CameraForward :type "Vector Structure") (`Camera Forward 2` :type "Vector Structure"))
  (`self.RUNONSERVER Attack` Instigator OwnerTag CameraForward `Camera Forward 2`))

(event `RUNONSERVER Attack`
  (params (Instigator :type "/Game/BhandanaDesign/Actors/RPG_Actor Object Reference") (`Owner Tag` :type Name) (`Camera Forward` :type "Vector Structure") (`Camera Forward 2` :type "Vector Structure"))
  (bind _parentactor (`self.ParentActor`))
  (bind (_projectile_actor _projectile_size _number_of_projectiles) (`/Game/BhandanaDesign/Actors/OBJ_CustomMacros.Get Projectile Info` (`/Game/BhandanaDesign/Actors/RPG_Actor.CurrentWeapon` (`self.ParentActor`))))
  (bind (_outhit _returnvalue) (`KismetSystemLibrary.LineTraceSingleForObjects` `Camera Forward 2` `Camera Forward` (`self.Targets`) false (`|MakeArray` (`self.ParentActor`) :!type "Actor Object Reference") "None" true (struct :`R` 1.0 :`A` 1.0) (struct :`G` 1.0 :`A` 1.0) 9999.0))
  (for _ (range 1 (+ _number_of_projectiles 1))
    (bind (_projetile_rotation _firepoint) (`/Game/BhandanaDesign/Actors/OBJ_CustomMacros.CalculateBulletPath` _outhit _returnvalue (`/Game/BhandanaDesign/Actors/OBJ_CustomMacros.Get Weapon Barrel` (`self.Model`)) (`/Game/BhandanaDesign/Actors/RPG_Actor.CurrentWeapon` (`self.ParentActor`)))
      (:`  `
        (bind _returnvalue_2 (`|SpawnActorFromClass` _projectile_actor (`KismetMathLibrary.MakeTransform` _firepoint _projetile_rotation _projectile_size) "Undefined" "OverrideRootScale" null (`self.ParentActor`)))
        (`/Engine/EditorBlueprintResources/ActorMacros.Switch Has Authority`
          (:`Authority`
            (bind _output_get (set `self.finalDamage` (`KismetMathLibrary.RandomIntegerInRange` (`/Game/BhandanaDesign/Actors/RPG_Actor.gun MIN Damage` _parentactor) (`/Game/BhandanaDesign/Actors/RPG_Actor.gun MAX Damage` _parentactor))))
            (`self.UpdateBulletProperties` _output_get (`.AsDamageType` (`/Game/BhandanaDesign/Actors/OBJ_CustomMacros.Get Weapon Damage Type` (`/Game/BhandanaDesign/Actors/RPG_Actor.CurrentWeapon` Instigator))) _returnvalue_2 `Owner Tag`)))))))

(event `self.ReceiveBeginPlay`
  (bind _shield_mesh (`self.Shield Mesh`))
  (bind _shield_mesh_2 (`self.Shield Mesh`))
  (bind _tags (`self.Tags`))
  (bind ((`ShieldModel_18_B5C717A6484BF3F132CC4088AE01EEB9` _shieldmodel) (`ShieldMaterial_20_6222712944305FCD56C3689F1A36B3EF` _shieldmaterial) (`isActive_1_867286A44AB5E2B7FB083294132775FD` _isactive) (`ShieldHealth_13_7298EB114B75139F880AD79DDB27B9CE` _shieldhealth) (`ShieldHealthMax_15_B65913B74199E51E11C580AA12E2F41F` _shieldhealthmax)) (break `/Game/BhandanaDesign/VariableData/Structs/ST_ShieldData` (`.ShieldStats_85_E23A2CC641C9A943846F2E81E44B3E5D` (break `/Game/BhandanaDesign/VariableData/Structs/ST_WeaponData` (`/Game/BhandanaDesign/Actors/RPG_Actor.CurrentWeapon` (`self.ParentActor`))))))
  (bind (_shieldmodel_2 _shieldmaterial_2) (break `/Game/BhandanaDesign/VariableData/Structs/ST_ShieldData` (`.ShieldStats_85_E23A2CC641C9A943846F2E81E44B3E5D` (break `/Game/BhandanaDesign/VariableData/Structs/ST_WeaponData` (`/Game/BhandanaDesign/Actors/RPG_Actor.CurrentWeapon` (`self.ParentActor`))))))
  (bind _asrpg_actor (cast `/Game/BhandanaDesign/Actors/RPG_Actor` (`self.GetParentActor`))
    (:`then`
      (bind _output_get (set `self.ParentActor` _asrpg_actor))
      (`self.Multicast Initialize` _output_get)
      (bind (_weapon_model _weapon_skin) (`/Game/BhandanaDesign/Actors/OBJ_CustomMacros.Get Weapon Model Visuals` (`/Game/BhandanaDesign/Actors/RPG_Actor.CurrentWeapon` _output_get)))
      (`/Game/BhandanaDesign/Actors/OBJ_CustomMacros.UpdateWeaponAppearance` _weapon_model _weapon_skin self
        (:`  `
          (`self.OnUnequip`)
          (`PrimitiveComponent.SetMaterial` _shield_mesh 0 _shieldmaterial)
          (`MeshComponent.SetScalarParameterValueOnMaterials` _shield_mesh "HealthPercent" (`KismetMathLibrary.Conv_IntToDouble` (/ _shieldhealth _shieldhealthmax)))
          (`StaticMeshComponent.SetStaticMesh` (`self.Shield Mesh`) _shieldmodel)
          (`StaticMeshComponent.SetStaticMesh` _shield_mesh_2 _shieldmodel_2)
          (`PrimitiveComponent.SetMaterial` _shield_mesh_2 0 _shieldmaterial_2)
          (`self.Shield Handler` _isactive)
          (`KismetArrayLibrary.Array_Add` _tags (`/Game/BhandanaDesign/Actors/RPG_Actor.TagData` (`self.ParentActor`)))
          (set `self.Tags` _tags))))
    (:`CastFailed`
      (set `self.ParentActor` null))))

(event `Multicast Initialize`
  (params (Owner :type "Actor Object Reference"))
  (`self.SetOwner` Owner))

(event `UpdateSmallerData`)

(event `Shield Handler`
  (params (isActive :type Boolean) (`Weapon Data` :type "/Game/BhandanaDesign/VariableData/Structs/ST_WeaponData Structure"))
  (bind _shield_mesh (`self.Shield Mesh`))
  (bind _shield_mesh_2 (`self.Shield Mesh`))
  (`ActorComponent.SetActive` _shield_mesh_2 isActive false)
  (`SceneComponent.SetVisibility` _shield_mesh_2 isActive false)
  (if isActive
    (`PrimitiveComponent.SetCollisionEnabled` _shield_mesh "QueryOnly")
    (`PrimitiveComponent.SetMaterial` _shield_mesh 0 (`.ShieldMaterial_20_6222712944305FCD56C3689F1A36B3EF` (break `/Game/BhandanaDesign/VariableData/Structs/ST_ShieldData` (`.ShieldStats_85_E23A2CC641C9A943846F2E81E44B3E5D` (break `/Game/BhandanaDesign/VariableData/Structs/ST_WeaponData` `Weapon Data`)))))
    (`SceneComponent.SetVisibility` _shield_mesh true false)
    (`self.OnActivateShield`)
    (else
      (`PrimitiveComponent.SetCollisionEnabled` _shield_mesh "NoCollision")
      (`self.OnDeactivateShield`))))

(event `OnActivateShield`)

(event `OnDeactivateShield`)

(event `self.ReceiveAnyDamage`
  (params (Damage :type "Float (single-precision)") (DamageType :type "DamageType Object Reference") (InstigatedBy :type "Controller Object Reference") (DamageCauser :type "Actor Object Reference"))
  (bind _parentactor (`self.ParentActor`))
  (bind _currentweapon (`/Game/BhandanaDesign/Actors/RPG_Actor.CurrentWeapon` _parentactor))
  (bind _returnvalue (- (`.ShieldHealth_13_7298EB114B75139F880AD79DDB27B9CE` (break `/Game/BhandanaDesign/VariableData/Structs/ST_ShieldData` (`.ShieldStats_85_E23A2CC641C9A943846F2E81E44B3E5D` (break `/Game/BhandanaDesign/VariableData/Structs/ST_WeaponData` _currentweapon)))) (`KismetMathLibrary.Round` Damage)))
  (bind _returnvalue_2 (> _returnvalue 0))
  (`KismetSystemLibrary.PrintString` (`KismetStringLibrary.Conv_IntToString` _returnvalue))
  (if (not _returnvalue_2)
    (`self.Shield Handler` _returnvalue_2))
  (bind _new_weapon_data (`/Game/BhandanaDesign/Actors/OBJ_CustomMacros.Update Shield Health` _currentweapon _returnvalue)
    (:`  `
      (set `/Game/BhandanaDesign/Actors/RPG_Actor.CurrentWeapon` _new_weapon_data _parentactor)
      (`self.UpdateShieldHealth` (`self.ParentActor`))
      (`/Game/BhandanaDesign/Actors/RPG_Actor.Set Shield Recharge` (`self.ParentActor`)))))

(event `Recharge Shield Tick`
  (`self.UpdateShieldHealth` (`self.ParentActor`)))

(event `UpdateShieldHealth`
  (params (Parent :type "/Game/BhandanaDesign/Actors/RPG_Actor Object Reference"))
  (`/Engine/EditorBlueprintResources/StandardMacros.IsValid` Parent
    (:`Is Valid`
      (`MeshComponent.SetScalarParameterValueOnMaterials` (`self.Shield Mesh`) "HealthPercent" (/ (`KismetMathLibrary.Conv_IntToDouble` (`.ShieldHealth_13_7298EB114B75139F880AD79DDB27B9CE` (break `/Game/BhandanaDesign/VariableData/Structs/ST_ShieldData` (`.ShieldStats_85_E23A2CC641C9A943846F2E81E44B3E5D` (break `/Game/BhandanaDesign/VariableData/Structs/ST_WeaponData` (`/Game/BhandanaDesign/Actors/RPG_Actor.CurrentWeapon` Parent)))))) (`KismetMathLibrary.Conv_IntToDouble` (`/Game/BhandanaDesign/Actors/RPG_Actor.gun Shield Max` Parent)))))))

(event `Server Update Shield Health`
  (params (`Parent Actor` :type "/Game/BhandanaDesign/Actors/RPG_Actor Object Reference"))
  (`self.UpdateShieldHealth` `Parent Actor`))

(fn `UserConstructionScript`
  (bind _shield_mesh (`self.Shield Mesh`))
  (`SceneComponent.SetVisibility` _shield_mesh true false)
  (`PrimitiveComponent.SetCollisionEnabled` _shield_mesh "NoCollision"))