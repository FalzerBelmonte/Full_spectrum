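; Master Blueprint for melee weapons, handling the swing attack and its damage.
; Attack plays a montage on the owner, then sphere-traces from the Blade socket along the camera's forward vector, ignoring the owner.
; Hits run through the inherited CalculateBulletPath, and a DoOnce limits each swing to one server point-damage call with random damage in the given range.
; MulticastBeginADS sets the owner's ALS weapon mode.
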(event `/Game/BhandanaDesign/Interfaces/BPI_FS_WeaponInteractions.Attack`
  (params (Weapon :type "/Game/BhandanaDesign/VariableData/Structs/ST_WeaponData Structure") (MinDamage :type Integer) (MaxDamage :type Integer) (RaycastStart :type "Vector Structure") (RaycastEnd :type "Vector Structure") (TagData :type Name) (`Camera Forward Vector` :type "Vector Structure"))
  (bind _returnvalue (`self.GetOwner`))
  (bind _returnvalue_2 (`SceneComponent.GetSocketLocation` (`self.Model`) "Blade"))
  (message `/Game/BhandanaDesign/Interfaces/BPI_FS_Controller.Play_Montage` _returnvalue "/Game/BhandanaDesign/Animations/WIP_Montage.WIP_Montage")
  (bind _outhits (`KismetSystemLibrary.SphereTraceMulti` _returnvalue_2 (+ _returnvalue_2 (* `Camera Forward Vector` 250.0)) 50.0 "TraceTypeQuery5" false (`|MakeArray` _returnvalue)))
  (for _array_element _outhits
    (bind (_projetile_rotation _firepoint _should_i_do_damage_ _who_i_hit) (`/Game/BhandanaDesign/Actors/OBJ_CustomMacros.CalculateBulletPath` _array_element false (0.0 0.0 0.0) Weapon TagData)
      (:`Output with Hit`
        (if _should_i_do_damage_
          (`/Engine/EditorBlueprintResources/StandardMacros.DoOnce` false :!label _label
            (:`Completed`
              (`self.SERVER_Point Damage` _who_i_hit (`KismetMathLibrary.Conv_IntToDouble` (`KismetMathLibrary.RandomIntegerInRange` MinDamage MaxDamage)) _firepoint (struct) (`self.GetInstigatorController` (`self.GetOwner`)) self (`.AsDamageType` (`/Game/BhandanaDesign/Actors/OBJ_CustomMacros.Get Weapon Damage Type` Weapon)))))))))
  (goto _label :!via `Reset`))

(event `self.Multicast_Begin ADS`
  (message `/Game/BhandanaDesign/Interfaces/BPI_FS_Controller.Update_ALS_WeaponMode` (`self.GetOwner`) "NewEnumerator5"))

(fn `UserConstructionScript`
  (`parent.UserConstructionScript`))