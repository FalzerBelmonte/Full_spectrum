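; Dual pistols weapon that alternates shots between the main gun and an offhand BP_OffhandWeapon child actor using a FlipFlop.
; Each attack line-traces along the camera aim, then spawns the current weapon's projectiles from that gun's barrel.
; Authority rolls random damage from the firing gun's stats and applies it to each bullet.
; Equip events move the second gun, found by GetActorOfClass, between active and inactive mesh sockets, starting unequipped.
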(event `self.ReceiveBeginPlay`
  (`parent.ReceiveBeginPlay`)
  (`self.OnUnequip`))

(event `DualPisols Attack`
  (params (Instigator :type "/Game/BhandanaDesign/Actors/RPG_Actor Object Reference") (`Owner Tag` :type Name) (`Camera Forward` :type "Vector Structure") (`Camera Forward 2` :type "Vector Structure"))
  (bind _currentweapon (`/Game/BhandanaDesign/Actors/RPG_Actor.CurrentWeapon` Instigator))
  (bind _currentweapon_2 (`/Game/BhandanaDesign/Actors/RPG_Actor.CurrentWeapon` Instigator))
  (bind (_projectile_actor _projectile_size _number_of_projectiles) (`/Game/BhandanaDesign/Actors/OBJ_CustomMacros.Get Projectile Info` _currentweapon))
  (bind (_min_damage _max_damage) (`/Game/BhandanaDesign/Actors/OBJ_CustomMacros.Get Weapon Damage` _currentweapon_2))
  (bind _currentweapon_3 (`/Game/BhandanaDesign/Actors/RPG_Actor.CurrentWeapon` (`self.ParentActor`)))
  (bind (_projectile_actor_2 _projectile_size_2 _number_of_projectiles_2) (`/Game/BhandanaDesign/Actors/OBJ_CustomMacros.Get Projectile Info` _currentweapon_3))
  (bind _isa (`/Engine/EditorBlueprintResources/StandardMacros.FlipFlop`)
    (:`A`
      _)
    (:`B`
      _))
  (bind (_outhit _returnvalue) (`KismetSystemLibrary.LineTraceSingleForObjects` `Camera Forward 2` `Camera Forward` (`self.Targets`) false (`|MakeArray` (`self.ParentActor`) :!type "Actor Object Reference") "None" true (struct :`R` 1.0 :`A` 1.0) (struct :`G` 1.0 :`A` 1.0) 9999.0))
  (if _isa
    (for _ (range 1 (+ _number_of_projectiles 1))
      (bind (_projetile_rotation _firepoint) (`/Game/BhandanaDesign/Actors/OBJ_CustomMacros.CalculateBulletPath` _outhit _returnvalue (`/Game/BhandanaDesign/Actors/OBJ_CustomMacros.Get Weapon Barrel` (`self.Model`)) _currentweapon)
        (:`  `
          (bind _returnvalue_2 (`|SpawnActorFromClass` _projectile_actor (`KismetMathLibrary.MakeTransform` _firepoint _projetile_rotation _projectile_size) "Undefined" "OverrideRootScale" self Instigator))
          (`/Engine/EditorBlueprintResources/ActorMacros.Switch Has Authority`
            (:`Authority`
              (bind _output_get (set `self.finalDamage` (`KismetMathLibrary.RandomIntegerInRange` _min_damage _max_damage)))
              (`self.UpdateBulletProperties` _output_get (`.AsDamageType` (`/Game/BhandanaDesign/Actors/OBJ_CustomMacros.Get Weapon Damage Type` _currentweapon_2)) _returnvalue_2 `Owner Tag`))))))
    (else
      (bind _asbp_offhand_weapon (cast `/Game/BhandanaDesign/Actors/Weapons/BP_OffhandWeapon` (`ChildActorComponent.ChildActor` (`self.Offhand`))))
      (for _ (range 1 (+ _number_of_projectiles_2 1))
        (bind (_projetile_rotation_2 _firepoint_2) (`/Game/BhandanaDesign/Actors/OBJ_CustomMacros.CalculateBulletPath` _outhit _returnvalue (`/Game/BhandanaDesign/Actors/OBJ_CustomMacros.Get Weapon Barrel` (`/Game/BhandanaDesign/Actors/Weapons/BP_OffhandWeapon.MODEL` _asbp_offhand_weapon)) _currentweapon_3)
          (:`  `
            (bind _returnvalue_3 (`|SpawnActorFromClass` _projectile_actor_2 (`KismetMathLibrary.MakeTransform` _firepoint_2 _projetile_rotation_2 _projectile_size_2) "Undefined" "OverrideRootScale" self Instigator))
            (set `/Game/BhandanaDesign/Actors/Projectiles/BP_Projectile.TagData` "None" _returnvalue_3)
            (`/Engine/EditorBlueprintResources/ActorMacros.Switch Has Authority`
              (:`Authority`
                (bind (_weapon_stats_level _weapon_stats_mindamage _weapon_stats_maxdamage _weapon_stats_damagetype) (break `/Game/BhandanaDesign/VariableData/Structs/ST_WeaponStats` (`/Game/BhandanaDesign/Actors/Weapons/BP_OffhandWeapon.Weapon Stats` _asbp_offhand_weapon)))
                (bind _output_get_2 (set `self.finalDamage` (`KismetMathLibrary.RandomIntegerInRange` _weapon_stats_mindamage _weapon_stats_maxdamage)))
                (`self.UpdateBulletProperties` _output_get_2 (`/Game/BhandanaDesign/Actors/OBJ_CustomMacros.Get DamageType` _weapon_stats_damagetype) _returnvalue_3)))))))))

(event `self.RUNONSERVER Attack`
  (params (Instigator :type "/Game/BhandanaDesign/Actors/RPG_Actor Object Reference") (`Owner Tag` :type Name) (`Camera Forward` :type "Vector Structure") (`Camera Forward 2` :type "Vector Structure"))
  (`self.DualPisols Attack` Instigator `Owner Tag` `Camera Forward` `Camera Forward 2`))

(event `self.OnUnequip`
  (`self.UnequipOffhand`))

(event `self.OnEquip`
  (`self.EquipOffhand`))

(fn `UserConstructionScript`
  (`parent.UserConstructionScript`))