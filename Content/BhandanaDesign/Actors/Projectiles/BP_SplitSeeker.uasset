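; BP_SplitSeeker is a projectile that zigzags vertically in flight.
; Its CustomBehaviorOffBeginPlay event starts a short looping timer and stores the current velocity in MEMVelocity.
; Each timer tick flip-flops the ProjectileMovement velocity between that stored velocity plus an upward offset and plus an equal downward one.
; Despite the name, this graph contains no splitting or target-seeking logic.
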(event `self.Custom Behavior off BeginPlay`
  (`KismetSystemLibrary.K2_SetTimerDelegate` (delegate `Switch`) 0.3 true)
  (set `self.MEM_Velocity` (`self.GetVelocity`)))

(event `Switch`
  (bind _mem_velocity (`self.MEM_Velocity`))
  (`/Engine/EditorBlueprintResources/StandardMacros.FlipFlop`
    (:`A`
      (set `MovementComponent.Velocity` (+ _mem_velocity (0.0 0.0 200.0)) (`self.ProjectileMovement`)))
    (:`B`
      (set `MovementComponent.Velocity` (+ _mem_velocity (0.0 0.0 -200.0)) (`self.ProjectileMovement`)))))

(fn `UserConstructionScript`
  (`parent.UserConstructionScript`))