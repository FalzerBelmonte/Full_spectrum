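; Shuriken projectile that damages what it hits and sticks into it, extending a parent projectile Blueprint.
; Model hits ignore the instigator, send server damage to Entity or Destructable components lacking the TagData tag, and clean up on those or other surfaces.
; Cleanup stops the spin, destroys the trail and attaches the shuriken to the hit component and bone, keeping its world transform.
; BeginPlay randomizes the model's pitch slightly.
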(event `self.Model.OnComponentHit`
  (params (HitComponent :type "PrimitiveComponent Object Reference") (OtherActor :type "Actor Object Reference") (OtherComp :type "PrimitiveComponent Object Reference") (NormalImpulse :type "Vector Structure") (Hit :type "HitResult Structure (by ref)"))
  (bind _returnvalue (`self.GetInstigator`))
  (set `self.REP_HitData` Hit)
  (set `self.StickPoint` OtherComp)
  (if (!= OtherActor _returnvalue)
    (if (or (`ActorComponent.ComponentHasTag` OtherComp "Entity") (`ActorComponent.ComponentHasTag` OtherComp "Destructable"))
      (if (not (`ActorComponent.ComponentHasTag` OtherComp (`self.TagData`)))
        (`self.Server Apply Damage` OtherActor (`KismetMathLibrary.Conv_IntToDouble` (`self.Damage`)) _returnvalue (`self.DamageType`) Hit)
        (`self.Cleanup`))
      (else
        (`self.Cleanup`)))))

(event `self.ReceiveBeginPlay`
  (bind _model (`self.Model`))
  (bind (_returnvalue_roll _returnvalue_pitch _returnvalue_yaw) (`KismetMathLibrary.BreakRotator` (`SceneComponent.K2_GetComponentRotation` _model)))
  (`parent.ReceiveBeginPlay`)
  (`SceneComponent.K2_SetWorldRotation` _model (`KismetMathLibrary.MakeRotator` _returnvalue_roll (+ _returnvalue_pitch (`KismetMathLibrary.RandomFloatInRange` -10.0 10.0)) _returnvalue_yaw) false false))

(event `self.Cleanup`
  (bind (_rep_hitdata_bblockinghit _rep_hitdata_binitialoverlap _rep_hitdata_time _rep_hitdata_distance _rep_hitdata_location _rep_hitdata_impactpoint _rep_hitdata_normal _rep_hitdata_impactnormal _rep_hitdata_physmat _rep_hitdata_hitactor _rep_hitdata_hitcomponent _rep_hitdata_hitbonename) (`GameplayStatics.BreakHitResult` (`self.REP_HitData`)))
  (`parent.Cleanup`)
  (set `RotatingMovementComponent.RotationRate` (struct) (`self.RotatingMovement`))
  (`ActorComponent.K2_DestroyComponent` (`self.BulletTrail`))
  (`self.K2_AttachToComponent` (`self.StickPoint`) _rep_hitdata_hitbonename "KeepWorld" "KeepWorld" "KeepWorld"))

(fn `UserConstructionScript`
  (`parent.UserConstructionScript`))