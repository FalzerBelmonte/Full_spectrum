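; BP_Healing_Projectile is a projectile that heals or damages what it hits, depending on component tags.
; Its Model ignores the instigator and, on hit, checks for an Entity or Destructable tag.
; Components also carrying TagData receive a tenth of Damage as negative damage, others full damage, via ServerApplyDamage.
; Any non-instigator hit calls Cleanup, and debug prints report each outcome.
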(event `self.Model.OnComponentHit`
  (params (HitComponent :type "PrimitiveComponent Object Reference") (OtherActor :type "Actor Object Reference") (OtherComp :type "PrimitiveComponent Object Reference") (NormalImpulse :type "Vector Structure") (Hit :type "HitResult Structure (by ref)"))
  (bind _returnvalue (`self.GetInstigator`))
  (bind _damagetype (`self.DamageType`))
  (`KismetSystemLibrary.PrintString` (`KismetSystemLibrary.GetDisplayName` OtherActor))
  (if (!= OtherActor _returnvalue)
    (if (or (`ActorComponent.ComponentHasTag` OtherComp "Entity") (`ActorComponent.ComponentHasTag` OtherComp "Destructable"))
      (if (`ActorComponent.ComponentHasTag` OtherComp (`self.TagData`))
        (`self.Server Apply Damage` OtherActor (/ (`KismetMathLibrary.Conv_IntToDouble` (* (`self.Damage`) -1)) 10.0) _returnvalue _damagetype Hit)
        (else
          (`self.Server Apply Damage` OtherActor (`KismetMathLibrary.Conv_IntToDouble` (`self.Damage`)) _returnvalue _damagetype Hit)))
      (`self.Cleanup`)
      (`KismetSystemLibrary.PrintString` "Dealt Damage" true true (struct :`R` 1.0 :`B` 0.042102 :`A` 1.0))
      (else
        (`KismetSystemLibrary.PrintString` "Not an Entity")
        (`self.Cleanup`)))
    (else
      (`KismetSystemLibrary.PrintString` "Hit owner"))))

(event `self.ReceiveBeginPlay`
  (`PrimitiveComponent.IgnoreActorWhenMoving` (`self.Model`) (`self.GetInstigator`) true))

(fn `UserConstructionScript`
  (`parent.UserConstructionScript`))