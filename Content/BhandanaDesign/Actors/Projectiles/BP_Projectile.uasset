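; Projectile actor that deals point damage on hit to components tagged Entity or Destructable, sparing its instigator and allies.
; TagData marks allies: BeginPlay makes the Model ignore actors with that tag, and hits on components carrying it deal no damage.
; Damage goes through the ServerApplyDamage event, passing SpawnLocation as hit direction.
; Damaging or non-entity hits trigger Cleanup, which hides and stops the projectile without destroying it.
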(event `Cleanup`
  (bind _model (`self.Model`))
  (bind _projectilemovement (`self.ProjectileMovement`))
  ;[1 1 1] Removes Self
  (`SceneComponent.SetVisibility` _model false false)
  (`PrimitiveComponent.SetCollisionEnabled` _model "NoCollision")
  (set `ProjectileMovementComponent.MaxSpeed` 0.0 _projectilemovement)
  (set `MovementComponent.Velocity` (0.0 0.0 0.0) _projectilemovement))

(event `self.Model.OnComponentHit`
  (params (HitComponent :type "PrimitiveComponent Object Reference") (OtherActor :type "Actor Object Reference") (OtherComp :type "PrimitiveComponent Object Reference") (NormalImpulse :type "Vector Structure") (Hit :type "HitResult Structure (by ref)"))
  (bind _returnvalue (`self.GetInstigator`))
  (`KismetSystemLibrary.PrintString` (`KismetSystemLibrary.GetDisplayName` OtherActor))
  (if (!= OtherActor _returnvalue)
    (if (or (`ActorComponent.ComponentHasTag` OtherComp "Entity") (`ActorComponent.ComponentHasTag` OtherComp "Destructable"))
      (if (`ActorComponent.ComponentHasTag` OtherComp (`self.TagData`))
        (`KismetSystemLibrary.PrintString` "Hit an ally")
        (else
          (`self.Server Apply Damage` OtherActor (`KismetMathLibrary.Conv_IntToDouble` (`self.Damage`)) _returnvalue (`self.DamageType`) Hit)
          (`self.Cleanup`)
          (`KismetSystemLibrary.PrintString` "Dealt Damage" true true (struct :`R` 1.0 :`B` 0.042102 :`A` 1.0))))
      (else
        (`KismetSystemLibrary.PrintString` "Not an Entity")
        (`self.Cleanup`)))
    (else
      (`KismetSystemLibrary.PrintString` "Hit owner"))))

(event `Server Apply Damage`
  (params (`Damaged Actor` :type "Actor Object Reference") (`Base Damage` :type "Float (double-precision)") (`Damage Causer` :type "Actor Object Reference") (`Damage Type` :type "DamageType Class Reference") (`Hit Info` :type "HitResult Structure"))
  (`GameplayStatics.ApplyPointDamage` `Damaged Actor` `Base Damage` (`self.SpawnLocation`) `Hit Info` null `Damage Causer` `Damage Type`))

(event `self.ReceiveBeginPlay`
  (bind _outactors (`GameplayStatics.GetAllActorsWithTag` (`self.TagData`)))
  (for _array_element _outactors
    (`PrimitiveComponent.IgnoreActorWhenMoving` (`self.Model`) _array_element true)))

(fn `UserConstructionScript`)