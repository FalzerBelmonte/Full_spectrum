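; Projectile Blueprint that turns one shot into a three-way spread by spawning two secondary projectiles alongside itself.
; After the parent BeginPlay, a loop spawns the SecondaryProjectiles class at its own location, yawed five degrees to either side.
; Both spawns receive this projectile's owner, tag data and damage, with the damage type fixed to BP_NormalDamage.
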(event `self.ReceiveBeginPlay`
  (bind (_returnvalue_location _returnvalue_rotation _returnvalue_scale) (`KismetMathLibrary.BreakTransform` (`self.GetTransform`)))
  (`parent.ReceiveBeginPlay`)
  (for _index (range 2)
    (`|SpawnActorFromClass` (`self.Secondary Projectiles`) (`KismetMathLibrary.MakeTransform` _returnvalue_location (`KismetMathLibrary.MakeRotator` (.roll _returnvalue_rotation) (.pitch _returnvalue_rotation) (+ (.yaw _returnvalue_rotation) (select `int` _index :`0` -5.0 :`1` 5.0 :!type "Float (single-precision)"))) _returnvalue_scale) "Undefined" "OverrideRootScale" (`self.GetOwner`) (`self.TagData`) (`self.Damage`) "/Game/BhandanaDesign/Widgets/BP_NormalDamage.BP_NormalDamage_C" (`self.K2_GetActorLocation`) null)))

(fn `UserConstructionScript`
  (`parent.UserConstructionScript`))