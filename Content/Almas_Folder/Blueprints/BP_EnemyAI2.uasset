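; Enemy AI character with a montage-driven melee attack and player health handling.
; MeleeAttack plays AM_AI_Melee and, on its notify, sphere-traces forward from the hand_weapon socket with persistent debug drawing, then applies damage to the hit actor.
; The enemy's own AnyDamage event subtracts incoming damage from the player's Person health, prints it, and destroys the player when health equals exactly zero.
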(event `self.ReceiveAnyDamage`
  (params (Damage :type "Float (single-precision)") (DamageType :type "DamageType Object Reference") (InstigatedBy :type "Controller Object Reference") (DamageCauser :type "Actor Object Reference"))
  (bind _asperson (cast `/Game/Blueprints/Character/Person` (`GameplayStatics.GetPlayerCharacter` 0)))
  (bind _output_get (set `/Game/Blueprints/Character/Person.Health` (- (`/Game/Blueprints/Character/Person.Health` _asperson) Damage) _asperson))
  (`KismetSystemLibrary.PrintString` (`KismetStringLibrary.Conv_DoubleToString` _output_get))
  (if (== (`/Game/Blueprints/Character/Person.Health` _asperson) 0.0)
    (`KismetSystemLibrary.PrintString` "Player died")
    (`self.K2_DestroyActor` _asperson)))

(event `/Game/Almas_Folder/Blueprints/Interface/INT_Enemy.MeleeAttack`
  (bind _returnvalue (`SceneComponent.GetSocketLocation` (`self.Mesh`) "hand_weapon"))
  (`|PlayMontage` (`self.Mesh`) "/Game/Animation/AI/Punch/AM_AI_Melee.AM_AI_Melee"
    (:`OnNotifyBegin`
      (bind _outhit (`KismetSystemLibrary.SphereTraceSingle` :`Start` _returnvalue :`End` (+ _returnvalue (* (`KismetMathLibrary.GetForwardVector` (`self.K2_GetActorRotation`)) 50.0)) :`Radius` 40.0 :`TraceChannel` "TraceTypeQuery2" :`DrawDebugType` "Persistent"))
      (`GameplayStatics.ApplyDamage` (`.HitActor` (`GameplayStatics.BreakHitResult` _outhit)) 10.0))))

(fn `UserConstructionScript`)