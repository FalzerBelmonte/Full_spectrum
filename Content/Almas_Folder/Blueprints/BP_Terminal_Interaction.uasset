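; BP_Terminal_Interaction is an interactable terminal that shows a level selection UI to a nearby local player.
; When a local INT_Player actor enters its box, it creates WBP_LevelSelection, runs the widget's near-player step and adds it to the viewport.
; Interact advances the widget to its second step.
; Leaving the box removes and clears the widget.
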(event `/Game/Almas_Folder/Blueprints/Interface/INT_Interact.Interact`
  (`/Game/Almas_Folder/Widgets/WBP_LevelSelection.Step 2: After they Interact` (`self.Terminal`)))

(event `self.Box.OnComponentBeginOverlap`
  (params (OverlappedComponent :type "PrimitiveComponent Object Reference") (OtherActor :type "Actor Object Reference") (OtherComp :type "PrimitiveComponent Object Reference") (OtherBodyIndex :type Integer) (bFromSweep :type Boolean) (SweepResult :type "HitResult Structure (by ref)"))
  (bind _returnvalue (`self.GetInstigatorController` OtherActor))
  (if (`KismetSystemLibrary.DoesImplementInterface` OtherActor "/Game/Almas_Folder/Blueprints/Interface/INT_Player.INT_Player_C")
    (`/Engine/EditorBlueprintResources/StandardMacros.IsValid` (`self.Terminal`)
      (:`Is Not Valid`
        (`/Engine/EditorBlueprintResources/StandardMacros.IsValid` _returnvalue
          (:`Is Valid`
            (if (`Controller.IsLocalPlayerController` _returnvalue)
              (bind _asplayer_controller (cast `PlayerController` _returnvalue))
              (bind _returnvalue_2 (`|CreateWidget` "/Game/Almas_Folder/Widgets/WBP_LevelSelection.WBP_LevelSelection_C" _asplayer_controller))
              (bind _output_get (set `self.Terminal` _returnvalue_2))
              (`/Game/Almas_Folder/Widgets/WBP_LevelSelection.Step 1: When Player Is Near` _output_get)
              (`UserWidget.AddToViewport` _output_get 1)
              (`UserWidget.AddToViewport` _returnvalue_2 1))))))))

(event `self.Box.OnComponentEndOverlap`
  (params (OverlappedComponent :type "PrimitiveComponent Object Reference") (OtherActor :type "Actor Object Reference") (OtherComp :type "PrimitiveComponent Object Reference") (OtherBodyIndex :type Integer))
  (bind _returnvalue (`self.GetInstigatorController` OtherActor))
  (bind _terminal (`self.Terminal`))
  (if (`KismetSystemLibrary.DoesImplementInterface` OtherActor "/Game/Almas_Folder/Blueprints/Interface/INT_Player.INT_Player_C")
    (`/Engine/EditorBlueprintResources/StandardMacros.IsValid` _returnvalue
      (:`Is Valid`
        (if (`Controller.IsLocalPlayerController` _returnvalue)
          (`/Engine/EditorBlueprintResources/StandardMacros.IsValid` _terminal
            (:`Is Valid`
              (`Widget.RemoveFromParent` _terminal)
              (set `self.Terminal` null))))))))

(fn `UserConstructionScript`)