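; Test NPC that offers stepped dialogue to a nearby player and blends the camera to itself on interaction.
; Its trigger creates the dialogue widget for overlapping local players implementing INT_Player, and removes it on exit, resetting progress.
; Each Interact shows the next MyText line, then opens the widget's options once lines run out and restarts the count.
; ResetCameraTrigger is called when dialogue finishes or the player leaves, but is empty here.
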(event `ResetCameraTrigger`)

(event `/Game/Almas_Folder/Blueprints/Interface/INT_Interact.Interact`
  (bind _dialogue (`self.Dialogue`))
  (bind _mytext (`self.MyText`))
  (bind _returnvalue (`KismetArrayLibrary.Array_Length` _mytext))
  (`PlayerController.SetViewTargetWithBlend` (`GameplayStatics.GetPlayerController` 0) self 0.5 "VTBlend_Linear" 0.0 true)
  (`/Engine/EditorBlueprintResources/StandardMacros.IsValid` _dialogue
    (:`Is Valid`
      (`/Game/Almas_Folder/Widgets/WBP_NPCDialogue.Step2` _dialogue)
      (set `/Game/Almas_Folder/Widgets/WBP_NPCDialogue.DialogueText` (`|GetArrayItem` _mytext (`self.DialogueStep`)) (`self.Dialogue`))
      (bind _result (`/Engine/EditorBlueprintResources/StandardMacros.IncrementInt` (`self.DialogueStep`))
        (:`  `
          (if (> _result _returnvalue)
            (set `self.DialogueStep` _returnvalue)
            (`self.Open Options`)
            (set `self.DialogueStep` 0)
            (`self.ResetCameraTrigger`)))))))

(event `Open Options`
  (`/Game/Almas_Folder/Widgets/WBP_NPCDialogue.Show Options` (`self.Dialogue`)))

(event `self.Trigger.OnComponentBeginOverlap`
  (params (OverlappedComponent :type "PrimitiveComponent Object Reference") (OtherActor :type "Actor Object Reference") (OtherComp :type "PrimitiveComponent Object Reference") (OtherBodyIndex :type Integer) (bFromSweep :type Boolean) (SweepResult :type "HitResult Structure (by ref)"))
  (bind _returnvalue (`self.GetInstigatorController` OtherActor))
  (if (`KismetSystemLibrary.DoesImplementInterface` OtherActor "/Game/Almas_Folder/Blueprints/Interface/INT_Player.INT_Player_C")
    (`/Engine/EditorBlueprintResources/StandardMacros.IsValid` (`self.Dialogue`)
      (:`Is Not Valid`
        (`/Engine/EditorBlueprintResources/StandardMacros.IsValid` _returnvalue
          (:`Is Valid`
            (if (`Controller.IsLocalPlayerController` _returnvalue)
              (bind _asplayer_controller (cast `PlayerController` _returnvalue))
              (bind _returnvalue_2 (`|CreateWidget` "/Game/Almas_Folder/Widgets/WBP_NPCDialogue.WBP_NPCDialogue_C" _asplayer_controller))
              (bind _output_get (set `self.Dialogue` _returnvalue_2))
              (`/Game/Almas_Folder/Widgets/WBP_NPCDialogue.Step1` _output_get)
              (`UserWidget.AddToViewport` _output_get 8)
              (`UserWidget.AddToViewport` _returnvalue_2 8))))))))

(event `self.Trigger.OnComponentEndOverlap`
  (params (OverlappedComponent :type "PrimitiveComponent Object Reference") (OtherActor :type "Actor Object Reference") (OtherComp :type "PrimitiveComponent Object Reference") (OtherBodyIndex :type Integer))
  (bind _returnvalue (`self.GetInstigatorController` OtherActor))
  (bind _dialogue (`self.Dialogue`))
  (if (`KismetSystemLibrary.DoesImplementInterface` OtherActor "/Game/Almas_Folder/Blueprints/Interface/INT_Player.INT_Player_C")
    (`/Engine/EditorBlueprintResources/StandardMacros.IsValid` _returnvalue
      (:`Is Valid`
        (if (`Controller.IsLocalPlayerController` _returnvalue)
          (`/Engine/EditorBlueprintResources/StandardMacros.IsValid` _dialogue
            (:`Is Valid`
              (`Widget.RemoveFromParent` _dialogue)
              (set `self.Dialogue` null)
              (set `self.DialogueStep` 0)
              (`self.ResetCameraTrigger`))))))))

(fn `UserConstructionScript`)