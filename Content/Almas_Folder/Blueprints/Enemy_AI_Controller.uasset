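; AI controller for BP_EnemyAI2 that runs the BT_Enemy behavior tree and feeds it patrol and perception data.
; On BeginPlay it seeds the blackboard with the pawn's patrol path settings and a starting direction.
; Perception updates pass each actor's stimuli to CompleteSense, which identifies senses by array index rather than type.
; The first stimulus drives CanSeePlayer, and the second drives isLooking and TargetLocation.
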(event `self.ReceiveBeginPlay`
  (bind _returnvalue (`AIBlueprintHelperLibrary.GetBlackboard` null))
  (`self.RunBehaviorTree` "/Game/Blueprints/AI/Blackboard/BT_Enemy.BT_Enemy")
  (bind _asbp_enemy_ai2 (cast `/Game/Almas_Folder/Blueprints/BP_EnemyAI2` (`self.K2_GetPawn`)))
  (bind _output_get (set `self.MyPawn` _asbp_enemy_ai2))
  (`BlackboardComponent.SetValueAsBool` (`AIBlueprintHelperLibrary.GetBlackboard` null) "PathLoop" (`/Game/Almas_Folder/Blueprints/BP_PatrolPath.IsLooping` (`/Game/Almas_Folder/Blueprints/BP_EnemyAI2.PatrolPath` _output_get)))
  (`BlackboardComponent.SetValueAsInt` _returnvalue "Direction" 1)
  (`BlackboardComponent.SetValueAsFloat` _returnvalue "WaitTime" (`/Game/Almas_Folder/Blueprints/BP_PatrolPath.WaitTime` (`/Game/Almas_Folder/Blueprints/BP_EnemyAI2.PatrolPath` (`self.MyPawn`)))))

(event `self.AIPerception.OnPerceptionUpdated`
  (params (UpdatedActors :type "Array of Actor Object Reference (by ref)"))
  (for _array_element UpdatedActors
    (bind _info (`AIPerceptionComponent.GetActorsPerception` (`self.AIPerception`) _array_element))
    (`self.CompleteSense` (`.LastSensedStimuli` (break `ActorPerceptionBlueprintInfo` _info)))))

(fn `CompleteSense`
  (params (Array :type "Array of AIStimulus Structure"))
  (locals (Local_Sense :type "AIStimulus Structure"))
  (bind (_local_sense_age _local_sense_expirationage _local_sense_strength _local_sense_stimuluslocation _local_sense_receiverlocation _local_sense_tag _local_sense_bsuccessfullysensed) (break `AIStimulus` (`local.Local_Sense`)))
  (bind (_local_sense_age_2 _local_sense_expirationage_2 _local_sense_strength_2 _local_sense_stimuluslocation_2 _local_sense_receiverlocation_2 _local_sense_tag_2 _local_sense_bsuccessfullysensed_2) (break `AIStimulus` (`local.Local_Sense`)))
  (for (_array_element _array_index) Array
    (set `local.Local_Sense` _array_element)
    (switch `int` _array_index
      (:`0`
        (`BlackboardComponent.SetValueAsBool` (`AIBlueprintHelperLibrary.GetBlackboard` null) "CanSeePlayer" _local_sense_bsuccessfullysensed))
      (:`1`
        (`BlackboardComponent.SetValueAsBool` (`AIBlueprintHelperLibrary.GetBlackboard` null) "isLooking" _local_sense_bsuccessfullysensed_2)
        (`BlackboardComponent.SetValueAsVector` (`AIBlueprintHelperLibrary.GetBlackboard` null) "TargetLocation" _local_sense_stimuluslocation_2)))))

(fn `UserConstructionScript`)