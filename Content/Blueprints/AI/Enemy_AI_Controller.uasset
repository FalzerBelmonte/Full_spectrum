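; Enemy AI controller that runs the BT_Enemy behavior tree on its possessed pawn.
; On BeginPlay it casts the pawn to BP_EnemyAI2 and seeds the blackboard with that pawn's patrol path loop and wait settings plus an initial direction.
; Perception updates set the CanSeePlayer key from the sensed state of any actor implementing the INT_Player interface.
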(event `self.ReceiveBeginPlay`
  (bind _returnvalue (`AIBlueprintHelperLibrary.GetBlackboard` null))
  (`self.RunBehaviorTree` "/Game/Blueprints/AI/Blackboard/BT_Enemy.BT_Enemy")
  (bind _asbp_enemy_ai2 (cast `/Game/Blueprints/AI/BP_EnemyAI2` (`self.K2_GetPawn`)))
  (bind _output_get (set `self.MyPawn` _asbp_enemy_ai2))
  (`BlackboardComponent.SetValueAsBool` (`AIBlueprintHelperLibrary.GetBlackboard` null) "PathLoop" (`/Game/Blueprints/AI/BP_PatrolPath.IsLooping` (`/Game/Blueprints/AI/BP_EnemyAI2.PatrolPath` _output_get)))
  (`BlackboardComponent.SetValueAsInt` _returnvalue "Direction" 1)
  (`BlackboardComponent.SetValueAsFloat` _returnvalue "WaitTime" (`/Game/Blueprints/AI/BP_PatrolPath.WaitTime` (`/Game/Blueprints/AI/BP_EnemyAI2.PatrolPath` (`self.MyPawn`)))))

(event `self.AIPerception.OnTargetPerceptionUpdated`
  (params (Actor :type "Actor Object Reference") (Stimulus :type "AIStimulus Structure"))
  (if (`KismetSystemLibrary.DoesImplementInterface` Actor "/Game/Blueprints/Interface/INT_Player.INT_Player_C")
    (`BlackboardComponent.SetValueAsBool` (`AIBlueprintHelperLibrary.GetBlackboard` null) "CanSeePlayer" (`.bSuccessfullySensed` (break `AIStimulus` Stimulus)))))

(fn `UserConstructionScript`)