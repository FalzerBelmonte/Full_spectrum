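; Floating drone enemy that carries a weapon spawned from WeaponData and attached to its Scene component.
; A looping timer replays a timeline that moves Sphere2 vertically for the hover motion.
; AIAttack sends the gun an attack message aimed from its Barrel socket to just below the blackboard Target's bounds center.
; Damage drains Health, destroying gun and drone at zero, while getters expose AI and enemy data.
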(event `self.ReceiveBeginPlay`
  (`self.UpFloat`)
  (`KismetSystemLibrary.K2_SetTimerDelegate` (delegate `UpFloat`) 5.1 true)
  (bind _returnvalue (`|SpawnActorFromClass` (`/Game/BhandanaDesign/Actors/OBJ_CustomMacros.Get Weapon Actor` (`self.WeaponData`)) (`SceneComponent.K2_GetComponentToWorld` (`self.Scene`)) "Undefined" "OverrideRootScale" null self))
  (bind _output_get (set `self.SavedGun` _returnvalue))
  (`self.K2_AttachToComponent` _output_get (`self.Scene`) "None" "SnapToTarget" "SnapToTarget" "SnapToTarget" true)
  (set `self.MaxHealth` (`self.Health`)))

(event `UpFloat`
  (bind (_direction _newtrack_0) (`Timeline|Timeline_0` :!via `PlayFromStart`)
    (:`Update`
      (`SceneComponent.K2_AddRelativeLocation` (`self.Sphere2`) (`KismetMathLibrary.MakeVector` 0.0 0.0 _newtrack_0) true false))))

(event `/Game/BhandanaDesign/Interfaces/BPI_AI_Behaviors.AI_Attack`
  (bind _savedgun (`self.SavedGun`))
  (bind _weapondata (`self.WeaponData`))
  (bind (_weaponinformation _weaponvisuals _weaponstats) (break `/Game/BhandanaDesign/VariableData/Structs/ST_WeaponData` _weapondata))
  (bind _returnvalue_location (`KismetMathLibrary.BreakTransform` (`SceneComponent.GetSocketTransform` (`Actor.RootComponent` _savedgun) "Barrel" "RTS_World")))
  (bind _asactor (cast `Actor` (`BlackboardComponent.GetValueAsObject` (`AIBlueprintHelperLibrary.GetBlackboard` (`self.GetController`)) "Target")))
  (message `/Game/BhandanaDesign/Interfaces/BPI_FS_WeaponInteractions.Attack` _savedgun _weapondata (`.MINDamage_2_DEC9E0764C074C2D094463B881CF2443` (break `/Game/BhandanaDesign/VariableData/Structs/ST_WeaponStats` _weaponstats)) (`.MAXDamage_4_DDD17B174F75E5695580E98B4360A34A` (break `/Game/BhandanaDesign/VariableData/Structs/ST_WeaponStats` _weaponstats)) _returnvalue_location (- (`self.GetActorBounds` _asactor false false) (0.0 0.0 20.0)) (`self.TagData`) (`SceneComponent.GetForwardVector` (`self.Scene`))))

(event `self.ReceiveAnyDamage`
  (params (Damage :type "Float (single-precision)") (DamageType :type "DamageType Object Reference") (InstigatedBy :type "Controller Object Reference") (DamageCauser :type "Actor Object Reference"))
  (bind _output_get (set `self.Health` (- (`self.Health`) Damage)))
  (if (<= _output_get 0.0)
    (`self.K2_DestroyActor` (`self.SavedGun`))
    (`self.K2_DestroyActor`)))

(fn `AI_CheckDead`
  (returns (isDead :type Boolean))
  (return (<= (`self.Health`) 0.0)))

(fn `AI_GetAttackRange`
  (returns (`Attack Range` :type "Float (double-precision)"))
  (return (`self.AI_AttackRange`)))

(fn `AI_GetHealth`
  (returns (Health :type "Float (double-precision)"))
  (return (`self.Health`)))

(fn `AI_GetPersistance`
  (returns (`Time In Secondds` :type "Float (double-precision)"))
  (return (`self.AI_Persistence`)))

(fn `AI_GetWeapon`
  (returns (NewParam :type "/Game/BhandanaDesign/VariableData/Structs/ST_WeaponData Structure"))
  (return (`self.WeaponData`)))

(fn `GetEnemyData`
  (params (`Tag Data` :type Name))
  (returns (Name :type String) (Level :type Integer) (Health :type Integer) (`Max Health` :type Integer) (`Faction Tag` :type "/Game/BhandanaDesign/VariableData/Enums/TeamFaction Enum"))
  (return "Drone" 1 (`KismetMathLibrary.FTrunc` (`self.Health`)) (`KismetMathLibrary.FTrunc` (`self.MaxHealth`)) "NewEnumerator1"))

(fn `UserConstructionScript`)