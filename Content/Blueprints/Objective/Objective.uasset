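; World objective marker actor that shows its distance from a referenced character in meters.
; Each tick it scales the marker backing and text by clamped distance for readability and yaws and pitches the marker toward the player camera.
; A HUD widget is added when the objective fails to project to the screen and removed when it projects.
; The logic that would assign the character reference is unconnected.
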(event `self.ReceiveBeginPlay`)

(event `self.ReceiveTick`
  (params (DeltaSeconds :type "Float (single-precision)"))
  (bind _objective (`self.Objective`))
  (bind _returnvalue (`SceneComponent.K2_GetComponentLocation` _objective))
  (bind (_returnvalue_roll _returnvalue_pitch _returnvalue_yaw) (`KismetMathLibrary.BreakRotator` (`KismetMathLibrary.FindLookAtRotation` _returnvalue (`PlayerCameraManager.GetCameraLocation` (`GameplayStatics.GetPlayerCameraManager` 0)))))
  (bind _returnvalue_2 (`KismetMathLibrary.Vector_Distance` (`self.K2_GetActorLocation` (`self.Find character`)) _returnvalue))
  (bind _returnvalue_3 (`KismetMathLibrary.FClamp` (/ (`KismetMathLibrary.Hypotenuse` _returnvalue_2 (`KismetMathLibrary.Vector_Distance` _returnvalue (`SceneComponent.K2_GetComponentLocation` (`self.Cube`)))) 20.0) 50.0 1000.0))
  (`SceneComponent.SetWorldScale3D` (`self.ObjectiveMarkerBack`) (`KismetMathLibrary.Conv_DoubleToVector` (/ _returnvalue_3 80.0)))
  (`TextRenderComponent.SetWorldSize` (`self.TextRender`) _returnvalue_3)
  (`TextRenderComponent.K2_SetText` (`self.TextRender`) (`KismetTextLibrary.Conv_StringToText` (`KismetStringLibrary.Concat_StrStr` (`KismetStringLibrary.Conv_IntToString` (/ (`KismetMathLibrary.FTrunc` _returnvalue_2) 100)) "m")))
  (`SceneComponent.K2_SetWorldRotation` _objective (`KismetMathLibrary.MakeRotator` 0.0 _returnvalue_pitch _returnvalue_yaw) false false)
  (if (`.ReturnValue` (`WidgetLayoutLibrary.ProjectWorldLocationToWidgetPosition` (`GameplayStatics.GetPlayerController` 0) (`SceneComponent.K2_GetComponentLocation` (`self.Objective`))))
    (`Widget.RemoveFromParent` (stale _returnvalue_4))
    (set `self.IsLoaded` false)
    (elif (not (`self.IsLoaded`))
      (bind _returnvalue_4 (`|CreateWidget` "/Game/Almas_Folder/Widgets/HUD.HUD_C" (`GameplayStatics.GetPlayerController` 0)))
      (set `self.IsLoaded` true)
      (`UserWidget.AddToViewport` _returnvalue_4 0))))

(fn `UserConstructionScript`)