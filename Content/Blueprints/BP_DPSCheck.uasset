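; BP_DPSCheck is a damage test actor meant to measure damage per second.
; AnyDamage adds to DPS while Recording is set; otherwise it overwrites DPS and starts a one-second timer that prints and clears it.
; The graph never sets Recording true.
; Tick writes TotalHP to a TextRender, though damage never changes that value.
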(event `self.ReceiveBeginPlay`
  (`parent.ReceiveBeginPlay`))

(event `self.ReceiveTick`
  (params (DeltaSeconds :type "Float (single-precision)"))
  (`TextRenderComponent.K2_SetText` (`self.TextRender`) (`KismetTextLibrary.Conv_DoubleToText` (`self.Total HP`) "HalfToEven")))

(event `self.ReceiveAnyDamage`
  (params (Damage :type "Float (single-precision)") (DamageType :type "DamageType Object Reference") (InstigatedBy :type "Controller Object Reference") (DamageCauser :type "Actor Object Reference"))
  (if (`self.Recording`)
    (set `self.DPS` (+ (`self.DPS`) Damage))
    (else
      (set `self.Recording` false)
      (set `self.DPS` Damage)
      (`KismetSystemLibrary.K2_SetTimerDelegate` (delegate `DPSCheck`) 1.0))))

(event `DPSCheck`
  (`KismetSystemLibrary.PrintString` (`KismetStringLibrary.Conv_DoubleToString` (`self.DPS`)))
  (set `self.DPS` 0.0))

(fn `UserConstructionScript`
  (`parent.UserConstructionScript`))