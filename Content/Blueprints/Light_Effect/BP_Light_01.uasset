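; Flickering light fixture that cycles its light on and off, swapping the static mesh material to match.
; A looping BeginPlay timer toggles between the Static_Light macro and an off macro that zeroes intensity.
; Static_Light uses its own FlipFlop to alternate a steady switch-on with a brief delayed blink before staying lit.
; The construction script applies LightPower as the initial intensity.
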(event `FlickerLights`
  (bind _light_flickering (`self.Light_Flickering`))
  (`/Engine/EditorBlueprintResources/StandardMacros.FlipFlop`
    (:`A`
      (`self.Static_Light` _light_flickering _light_flickering _light_flickering _light_flickering))
    (:`B`
      (`self.NewMacro_0` _light_flickering))))

(event `self.ReceiveBeginPlay`
  (`KismetSystemLibrary.K2_SetTimerDelegate` (delegate `FlickerLights`) 2.0 true))

(fn `UserConstructionScript`
  (`LightComponent.SetIntensity` (`self.Light_Flickering`) (`self.Light Power`)))