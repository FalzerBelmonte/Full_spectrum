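; BP_Plate is a plate that fades out one randomly assigned door when an RPG_Actor stands on it.
; On BeginPlay it picks the door from the first three DoorReferences entries, using RandomInteger on LastIndex, so the array's final entry is never rolled.
; Overlap starts a five-second Delay, then calls FadeOut on the valid door if the actor is overlapping at that moment.
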(event `self.ReceiveBeginPlay`
  (bind _doorreferences (`self.DoorReferences`))
  (bind _output_get (set `self.Selector` (`KismetMathLibrary.RandomInteger` (`KismetArrayLibrary.Array_LastIndex` _doorreferences))))
  (set `self.AccessedDoor` (select `int` _output_get :`0` (`|GetArrayItem` _doorreferences) :`1` (`|GetArrayItem` _doorreferences 1) :`2` (`|GetArrayItem` _doorreferences 2))))

(event `self.ReceiveActorBeginOverlap`
  (params (OtherActor :type "Actor Object Reference"))
  (bind _accesseddoor (`self.AccessedDoor`))
  (cast `/Game/BhandanaDesign/Actors/RPG_Actor_2020-08-18-18-05-25_2020-08-18-18-56-45` OtherActor)
  (`KismetSystemLibrary.Delay` 5.0)
  (if (`self.IsOverlappingActor` OtherActor)
    (`/Engine/EditorBlueprintResources/StandardMacros.IsValid` _accesseddoor
      (:`Is Valid`
        (`/Game/Blueprints/BP_PlateDoor.FadeOut` _accesseddoor)))))

(fn `UserConstructionScript`)